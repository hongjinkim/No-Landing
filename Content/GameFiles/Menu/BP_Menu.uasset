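; BP_Menu is a menu actor with a widget component that moves the player's view between linked menu actors.
; On BeginPlay it binds to the transition event of its Menu_Widget, which passes an index into its LinkedMenus array.
; For a valid index, it disables its own collision, enables the target menu's, and blends the player's view target to that menu with an ease-in-out.
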(event `self.ReceiveBeginPlay`
  (bind _asmenu_widget (cast `/Game/GameFiles/Menu/widget/Menu_Widget` (`WidgetComponent.GetUserWidgetObject` (`self.Widget`))))
  (add `/Game/GameFiles/Menu/widget/Menu_Widget.TransitionToLinkedMenu` _asmenu_widget (delegate `OnTransitionBetweenMenus`)))

(event `OnTransitionBetweenMenus`
  (params (Menuindex :type Integer))
  (if (`KismetArrayLibrary.Array_IsValidIndex` (`self.LinkedMenus`) Menuindex)
    (`self.TransitionTo` (`|GetArrayItem` (`self.LinkedMenus`) Menuindex))))

(event `TransitionTo`
  (params (NewMenu :type "/Game/GameFiles/Menu/BP_Menu Object Reference"))
  (`self.SetActorEnableCollision` false)
  (`self.SetActorEnableCollision` NewMenu true)
  (`PlayerController.SetViewTargetWithBlend` (`GameplayStatics.GetPlayerController` 0) NewMenu 2.0 "VTBlend_EaseInOut" 2.0 false))

(fn `UserConstructionScript`)