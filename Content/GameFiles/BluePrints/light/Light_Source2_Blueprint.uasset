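; Light source Blueprint that tints its light toward a muted purple while the player character is doping.
; Each Tick casts the player to ALS_AnimMan_CharacterBP and, if IsDoping is set, sets a timeline's time from the normalized DopingTime.
; The timeline's track drives a color lerp on the LightComponent, so the tint follows the character's doping timer.
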(event `self.ReceiveTick`
  (params (DeltaSeconds :type "Float (single-precision)"))
  ;[1 1 1] light
  (`|ExecutionSequence`
    (:`then_0`
      (bind _asals_anim_man_character_bp (cast `/Game/AdvancedLocomotionV4/Blueprints/CharacterLogic/ALS_AnimMan_CharacterBP` (`GameplayStatics.GetPlayerCharacter` 0))))
    (:`then_1`
      (if (`/Game/AdvancedLocomotionV4/Blueprints/CharacterLogic/ALS_AnimMan_CharacterBP.is doping` _asals_anim_man_character_bp)
        (bind (_direction _newtrack_0) (`Timeline|타임라인_0` :`NewTime` (/ (`/Game/AdvancedLocomotionV4/Blueprints/CharacterLogic/ALS_AnimMan_CharacterBP.Doping time` _asals_anim_man_character_bp) 10.0) :!via `SetNewTime`)
          (:`Update`
            (`LightComponent.SetLightColor` (`self.LightComponent`) (`KismetMathLibrary.LinearColorLerp` (`KismetMathLibrary.MakeColor` 0.0) (`KismetMathLibrary.MakeColor` 0.580392 0.27451 0.494118) _newtrack_0) true)))))))

(fn `UserConstructionScript`)