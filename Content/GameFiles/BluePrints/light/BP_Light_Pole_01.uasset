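; BP_Light_Pole_01 is a light pole that changes its light color while the player character is doping.
; Each tick it casts the player pawn to BP_Character and, if IsDoping is set, scrubs a timeline to the character's DopingTime.
; The timeline's track blends the light between a base color and a muted pink-purple.
; It also prints the track value every tick.
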(event `self.ReceiveTick`
  (params (DeltaSeconds :type "Float (single-precision)"))
  ;[1 1 1] light
  (`|ExecutionSequence`
    (:`then_0`
      (bind _asbp_character (cast `/Game/AmplifyAnimationPack/Blueprints/Character/BP_Character` (`GameplayStatics.GetPlayerPawn` 0))))
    (:`then_1`
      (if (`/Game/AmplifyAnimationPack/Blueprints/Character/BP_Character.Is Doping` _asbp_character)
        (bind (_direction _newtrack_0) (`Timeline|Timeline_0` :`NewTime` (/ (`/Game/AmplifyAnimationPack/Blueprints/Character/BP_Character.DopingTime` _asbp_character) 1.0) :!via `SetNewTime`)
          (:`Update`
            (`LightComponent.SetLightColor` (`self.LightComponent0`) (`KismetMathLibrary.LinearColorLerp` (`KismetMathLibrary.MakeColor` 0.0) (`KismetMathLibrary.MakeColor` 0.580392 0.27451 0.494118) _newtrack_0) true)))))
    (:`then_3`
      (`KismetSystemLibrary.PrintString` (`KismetStringLibrary.Conv_DoubleToString` _newtrack_0)))))

(fn `UserConstructionScript`)