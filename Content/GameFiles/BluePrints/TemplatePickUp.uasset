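; Template pickup actor that shows a prompt widget while the player is in range and increases the player's Drug count when collected.
; On BeginPlay it fills the widget from the ItemInfo struct and binds to the player character's PickUpItem event.
; Trigger overlaps toggle the prompt and range flag that gate collection.
; Collection adds to Drug through a FrameNumber value, then hides the actor and disables its collision instead of destroying it.
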(event `self.ReceiveBeginPlay`
  (bind _iteminfo (`self.ItemInfo`))
  (bind _pickupreference (`self.PickUpReference`))
  (bind (_item _2dtexture _pickuptext) (break `/Game/GameFiles/Inventory/BP/Item_struc` _iteminfo))
  ;[1 1 1] EventBegin
  (bind _returnvalue (`|CreateWidget` "/Game/GameFiles/Inventory/UI/PickupText.PickupText_C"))
  (set `self.PickUpReference` _returnvalue)
  (setmembers `/Game/GameFiles/Inventory/BP/Item_struc` :`StructRef` _iteminfo :`Item` self)
  (set `/Game/GameFiles/Inventory/UI/PickupText.PickupActor` _item _pickupreference)
  (set `/Game/GameFiles/Inventory/UI/PickupText.PickupText` _pickuptext _pickupreference)
  (bind _asparent_char_char_bp (cast `/Game/GameFiles/BluePrints/ParentChar_CharBP` (`GameplayStatics.GetPlayerCharacter` 0)))
  (bind _output_get (set `self.CharacterReference` _asparent_char_char_bp))
  (add `/Game/GameFiles/BluePrints/ParentChar_CharBP.PickUpItem` _output_get (delegate `PickUpItem`)))

(event `self.Trigger.OnComponentBeginOverlap`
  (params (OverlappedComponent :type "PrimitiveComponent Object Reference") (OtherActor :type "Actor Object Reference") (OtherComp :type "PrimitiveComponent Object Reference") (OtherBodyIndex :type Integer) (bFromSweep :type Boolean) (SweepResult :type "HitResult Structure (by ref)"))
  (cast `/Game/GameFiles/BluePrints/ParentChar_CharBP` OtherActor)
  (`UserWidget.AddToViewport` (`self.PickUpReference`) 0)
  (set `self.IsInRange?` true))

(event `PickUpItem`
  ;[1 1 1] PickUpItem
  (if (and (`self.GetActorEnableCollision`) (`self.IsInRange?`))
    (bind _asparent_char_char_bp (cast `/Game/GameFiles/BluePrints/ParentChar_CharBP` (`GameplayStatics.GetPlayerCharacter` 0)))
    (set `/Game/GameFiles/BluePrints/ParentChar_CharBP.Drug` (+ (make `FrameNumber` 1) (`/Game/GameFiles/BluePrints/ParentChar_CharBP.Drug` _asparent_char_char_bp)) (`self.CharacterReference`))
    (`self.SetActorHiddenInGame` true)
    (`self.SetActorEnableCollision` false)))

(event `self.Trigger.OnComponentEndOverlap`
  (params (OverlappedComponent :type "PrimitiveComponent Object Reference") (OtherActor :type "Actor Object Reference") (OtherComp :type "PrimitiveComponent Object Reference") (OtherBodyIndex :type Integer))
  (cast `/Game/GameFiles/BluePrints/ParentChar_CharBP` OtherActor)
  (`Widget.RemoveFromParent` (`self.PickUpReference`))
  (set `self.IsInRange?` false))

(fn `UserConstructionScript`)