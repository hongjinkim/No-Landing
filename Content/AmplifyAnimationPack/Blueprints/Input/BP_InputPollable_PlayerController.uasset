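; Player controller that relays player input for movement, camera, combat, weapon, car and ability actions to the possessed pawn.
; On possess, it tries three casts in turn to cache the pawn and send it a possess event.
; Each action or axis binding then forwards to a matching event on that pawn, leaving gameplay logic out of the controller.
; A helper treats only keyboard keys as the active input device.
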(event `self.ReceivePossess`
  (params (PossessedPawn :type "Pawn Object Reference"))
  ;[1 1 1] OnPossess event
  (bind _asbp_character (cast `` PossessedPawn)
    (:`then`
      (bind _output_get (set `self.possessedPawn` _asbp_character)))
    (:`CastFailed`
      (bind _asbp_car_vehicle (cast `` PossessedPawn)
        (:`then`
          (bind _output_get_2 (set `self.possessedPawn` _asbp_car_vehicle)))
        (:`CastFailed`
          (bind _asbp_boat_actor (cast `` PossessedPawn))
          (bind _output_get_3 (set `self.possessedPawn` _asbp_boat_actor))))))
  (`/Game/AmplifyAnimationPack/Blueprints/Input/BPI_InputReciever.Input_PossessEvent` _output_get)
  (`/Game/AmplifyAnimationPack/Blueprints/Input/BPI_InputReciever.Input_PossessEvent` _output_get_2)
  (`/Game/AmplifyAnimationPack/Blueprints/Input/BPI_InputReciever.Input_PossessEvent` _output_get_3))

(event `InputAction|Interact`
  (params (Key :type "Key Structure"))
  ;[1 1 1] Character base inputs
  (:`Pressed`
    (`/Game/AmplifyAnimationPack/Blueprints/Input/BPI_InputReciever.Interact_InputEvent` (`self.possessedPawn`))))

(event `InputAction|WeaponReload`
  (params (Key :type "Key Structure"))
  ;[1 1 1] Weapon inputs
  (:`Pressed`
    (`/Game/AmplifyAnimationPack/Blueprints/Input/BPI_InputReciever.WeaponReload_InputEvent` (`self.possessedPawn`))))

(event `InputAxis|CarAccelerate`
  (params (AxisValue :type "Float (single-precision)"))
  ;[1 1 1] Car inputs
  (`/Game/AmplifyAnimationPack/Blueprints/Input/BPI_InputReciever.CarAccelerate_InputEvent` (`self.possessedPawn`) AxisValue))

(event `InputAxis|MoveForward`
  (params (AxisValue :type "Float (single-precision)"))
  ;[1 1 1] Character base inputs
  (`/Game/AmplifyAnimationPack/Blueprints/Input/BPI_InputReciever.MoveForward_InputEvent` (`self.possessedPawn`) AxisValue))

(event `InputAxis|MoveRight`
  (params (AxisValue :type "Float (single-precision)"))
  ;[1 1 1] Character base inputs
  (`/Game/AmplifyAnimationPack/Blueprints/Input/BPI_InputReciever.MoveRight_InputEvent` (`self.possessedPawn`) AxisValue))

(event `InputAction|Jump`
  (params (Key :type "Key Structure"))
  ;[1 1 1] Character base inputs
  (:`Pressed`
    (`/Game/AmplifyAnimationPack/Blueprints/Input/BPI_InputReciever.Jump_InputEvent` (`self.possessedPawn`))))

(event `InputAction|LightAttack`
  (params (Key :type "Key Structure"))
  ;[1 1 1] Character base inputs
  (:`Pressed`
    (`/Game/AmplifyAnimationPack/Blueprints/Input/BPI_InputReciever.LightAttack_InputEvent` (`self.possessedPawn`))))

(event `InputAction|WeaponShoot`
  (params (Key :type "Key Structure"))
  (bind _possessedpawn (`self.possessedPawn`))
  ;[1 1 1] Weapon inputs
  (:`Pressed`
    (`/Game/AmplifyAnimationPack/Blueprints/Input/BPI_InputReciever.WeaponShoot_InputEvent` _possessedpawn))
  (:`Released`
    (`/Game/AmplifyAnimationPack/Blueprints/Input/BPI_InputReciever.WeaponShootReleased_InputEvent` _possessedpawn)))

(event `InputAxis|Turn`
  (params (AxisValue :type "Float (single-precision)"))
  ;[1 1 1] Character base inputs
  (`/Game/AmplifyAnimationPack/Blueprints/Input/BPI_InputReciever.Turn_InputEvent` (`self.possessedPawn`) AxisValue))

(event `InputAction|Dodge`
  (params (Key :type "Key Structure"))
  ;[1 1 1] Character base inputs
  (:`Pressed`
    (`/Game/AmplifyAnimationPack/Blueprints/Input/BPI_InputReciever.Dodge_InputEvent` (`self.possessedPawn`))))

(event `InputAction|HeavyAttack`
  (params (Key :type "Key Structure"))
  ;[1 1 1] Character base inputs
  (:`Pressed`
    (`/Game/AmplifyAnimationPack/Blueprints/Input/BPI_InputReciever.HeavyAttack_InputEvent` (`self.possessedPawn`))))

(event `InputAction|WeaponAim`
  (params (Key :type "Key Structure"))
  (bind _possessedpawn (`self.possessedPawn`))
  ;[1 1 1] Weapon inputs
  (:`Pressed`
    (`/Game/AmplifyAnimationPack/Blueprints/Input/BPI_InputReciever.WeaponAim_InputEvent` _possessedpawn))
  (:`Released`
    (`/Game/AmplifyAnimationPack/Blueprints/Input/BPI_InputReciever.WeaponAimReleased_InputEvent` _possessedpawn)))

(event `InputAxis|LookUp`
  (params (AxisValue :type "Float (single-precision)"))
  ;[1 1 1] Character base inputs
  (`/Game/AmplifyAnimationPack/Blueprints/Input/BPI_InputReciever.LookUp_InputEvent` (`self.possessedPawn`) AxisValue))

(event `InputAction|LockOn`
  (params (Key :type "Key Structure"))
  ;[1 1 1] Character base inputs
  (:`Pressed`
    (`/Game/AmplifyAnimationPack/Blueprints/Input/BPI_InputReciever.LockOn_InputEvent` (`self.possessedPawn`))))

(event `InputAxis|WeaponEquip`
  (params (AxisValue :type "Float (single-precision)"))
  ;[1 1 1] Weapon inputs
  (`/Game/AmplifyAnimationPack/Blueprints/Input/BPI_InputReciever.WeaponEquip_InputEvent` (`self.possessedPawn`) AxisValue))

(event `InputAxis|SprintHold`
  (params (AxisValue :type "Float (single-precision)"))
  ;[1 1 1] Character base inputs
  (`/Game/AmplifyAnimationPack/Blueprints/Input/BPI_InputReciever.SprintHold_InputEvent` (`self.possessedPawn`) AxisValue))

(event `InputAxis|CrouchHold`
  (params (AxisValue :type "Float (single-precision)"))
  ;[1 1 1] Character base inputs
  (`/Game/AmplifyAnimationPack/Blueprints/Input/BPI_InputReciever.CrouchHold_InputEvent` (`self.possessedPawn`) AxisValue))

(event `InputAction|Blink`
  (params (Key :type "Key Structure"))
  ;[1 1 1] Weapon inputs
  (:`Pressed`
    (`/Game/AmplifyAnimationPack/Blueprints/Input/BPI_InputReciever.Blink_InputEvent` (`self.possessedPawn`))))

(event `InputAction|Activate`
  (params (Key :type "Key Structure"))
  ;[1 1 1] Weapon inputs
  (:`Pressed`
    (`/Game/AmplifyAnimationPack/Blueprints/Input/BPI_InputReciever.Activate_InputEvent` (`self.possessedPawn`))))

(event `InputAxis|JumpHold`
  (params (AxisValue :type "Float (single-precision)"))
  ;[1 1 1] Character base inputs
  (`/Game/AmplifyAnimationPack/Blueprints/Input/BPI_InputReciever.JumpHold_InputEvent` (`self.possessedPawn`) AxisValue))

(event `InputAction|Cancel`
  (params (Key :type "Key Structure"))
  (:`Pressed`
    (`/Game/AmplifyAnimationPack/Blueprints/Input/BPI_InputReciever.Cancel_InputEvent` (`self.possessedPawn`))))

(event `InputAction|Sprint`
  (params (Key :type "Key Structure"))
  ;[1 1 1] Character base inputs
  (:`Pressed`
    (`/Game/AmplifyAnimationPack/Blueprints/Input/BPI_InputReciever.SprintToggle_InputEvent` (`self.possessedPawn`))))

(event `InputAction|Drug`
  (params (Key :type "Key Structure"))
  (:`Pressed`
    (`/Game/AmplifyAnimationPack/Blueprints/Input/BPI_InputReciever.Drug_InputEvent` (`self.possessedPawn`))))

(event `InputAction|Crouch`
  (params (Key :type "Key Structure"))
  ;[1 1 1] Character base inputs
  (:`Pressed`
    (`/Game/AmplifyAnimationPack/Blueprints/Input/BPI_InputReciever.CrouchToggle_InputEvent` (`self.possessedPawn`))))

(event `InputAction|primary weapon`
  (params (Key :type "Key Structure"))
  (:`Pressed`
    (`/Game/AmplifyAnimationPack/Blueprints/Input/BPI_InputReciever.Input_PrimaryWeapon` (`self.possessedPawn`))))

(event `InputAction|secondary weapon`
  (params (Key :type "Key Structure"))
  (:`Pressed`
    (`/Game/AmplifyAnimationPack/Blueprints/Input/BPI_InputReciever.Input_SecondaryWeapon` (`self.possessedPawn`))))

(event `InputAction|special weapon`
  (params (Key :type "Key Structure"))
  (:`Pressed`
    (`/Game/AmplifyAnimationPack/Blueprints/Input/BPI_InputReciever.Input_SpecialWeapon` (`self.possessedPawn`))))

(fn `IsActiveInputDevice`
  (params (Key :type "Key Structure (by ref)"))
  (returns (`yes/no` :type Boolean))
  (return (`KismetInputLibrary.Key_IsKeyboardKey` Key)))

(fn `UserConstructionScript`)