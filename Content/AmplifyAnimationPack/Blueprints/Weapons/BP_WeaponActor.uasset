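; Base weapon actor that a player picks up through interaction, storing it and setting the character's pick-up animation direction.
; Fire, stop and attach hooks are empty stubs, alongside helpers for Niagara muzzle effects and line-trace shots.
; The shot shakes the camera, draws a debug trace and spawns an impact effect on hit.
; Trace-vector logic sketches a camera-or-weapon origin choice, but its nodes are unused.
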(event `Interact_1`
  (params (player :type "Object Object Reference"))
  (bind _wassuccessful (`self.Weapon_StoreWeapon` player self))
  (if _wassuccessful
    (`/Game/AmplifyAnimationPack/Animations/Character/Anim_Blueprints/Interfaces/BPI_AnimComunicator.Set_PickObjDirVal` (`/Game/AmplifyAnimationPack/Blueprints/Weapons/BP_WeaponActor.charAnimCommunicator` player) 0)))

(event `WeaponAttached Event`
  ;[1 1 1] Attachment custom events
)

(event `WeaponUnattached Event`
  ;[1 1 1] Attachment custom events
)

(fn `UserConstructionScript`)

(fn `Weapon_Fire`
  (params (weaponOwner :type "Object Object Reference")))

(fn `Weapon_LinetraceShot`
  (params (ownerRef :type "Object Object Reference"))
  (`PlayerCameraManager.StartCameraShake` :`self` (`GameplayStatics.GetPlayerCameraManager` 0))
  (bind _curentvalue (`/Game/AmplifyAnimationPack/Animations/Character/Anim_Blueprints/Interfaces/BPI_AnimComunicator.Get_CanShootInDirectionVal` (`/Game/AmplifyAnimationPack/Blueprints/Weapons/BP_WeaponActor.charAnimCommunicator` ownerRef)))
  (bind (_start _dir) (`self.Weapon_DecideLinetraceVectors` ownerRef _curentvalue))
  (bind (_outhit _returnvalue) (`KismetSystemLibrary.LineTraceSingleForObjects` :`Start` _start :`End` (+ _start (* _dir (`self.BulletRange`))) :`ObjectTypes` (`|MakeArray` "ObjectTypeQuery1" "ObjectTypeQuery2" :!type "EObjectTypeQuery Enum") :`DrawDebugType` "ForDuration"))
  (if _returnvalue
    (`|ExecutionSequence`
      (:`then_0`
        (`NiagaraFunctionLibrary.SpawnSystemAtLocation` "/Game/AmplifyAnimationPack/FX/NS_ImpactFX.NS_ImpactFX" (0.0 0.0 0.0) (struct) (1.0 1.0 1.0) true true "AutoRelease")))))

(fn `Weapon_MuzzleEffect`
  (`NiagaraFunctionLibrary.SpawnSystemAtLocation` (`self.MuzzleEffect`) (`SceneComponent.GetSocketLocation` (`self.Mesh`) "muzzleSocket") (struct) (1.0 1.0 1.0) true true "AutoRelease"))

(fn `Wepon_FireStopped`)