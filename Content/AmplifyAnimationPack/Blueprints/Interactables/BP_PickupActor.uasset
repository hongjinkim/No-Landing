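; BP_PickupActor is an interactable object that BP_Character can pick up, with weapon subclasses treated separately.
; Its PlayerDetector overlap registers it as the player's ObjectToInteract and shows or hides the pickup prompt.
; Interact switches the player to BP_InteractionState and stores non-weapons as ObjectPickedUp.
; It then sets the pickup animation's direction from the world-space Y offset and its interaction type from the height difference, via CharAnimCommunicator.
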(event `self.PlayerDetector.OnComponentBeginOverlap`
  (params (OverlappedComponent :type "PrimitiveComponent Object Reference") (OtherActor :type "Actor Object Reference") (OtherComp :type "PrimitiveComponent Object Reference") (OtherBodyIndex :type Integer) (bFromSweep :type Boolean) (SweepResult :type "HitResult Structure (by ref)"))
  (bind _asbp_character (cast `/Game/AmplifyAnimationPack/Blueprints/Character/BP_Character` OtherActor))
  (set `/Game/AmplifyAnimationPack/Blueprints/Character/BP_Character.objectToInteract` self _asbp_character)
  (`/Game/AmplifyAnimationPack/Blueprints/Character/BP_Character.UI_ShowInteractionUI` _asbp_character "Press E to Pickup object"))

(event `self.PlayerDetector.OnComponentEndOverlap`
  (params (OverlappedComponent :type "PrimitiveComponent Object Reference") (OtherActor :type "Actor Object Reference") (OtherComp :type "PrimitiveComponent Object Reference") (OtherBodyIndex :type Integer))
  (bind _asbp_character (cast `/Game/AmplifyAnimationPack/Blueprints/Character/BP_Character` OtherActor))
  (set `/Game/AmplifyAnimationPack/Blueprints/Character/BP_Character.objectToInteract` null _asbp_character)
  (`/Game/AmplifyAnimationPack/Blueprints/Character/BP_Character.UI_HideInteractionUI` _asbp_character))

(event `/Game/AmplifyAnimationPack/Blueprints/Interactables/BPI_Interactable.Interact`
  (params (player :type "/Game/AmplifyAnimationPack/Blueprints/Character/BP_Character Object Reference"))
  (bind _returnvalue (`self.K2_GetActorLocation` player))
  (bind (_returnvalue_x _returnvalue_y _returnvalue_z) (`KismetMathLibrary.BreakVector` (`self.K2_GetActorLocation`)))
  (bind _charanimcommunicator (`/Game/AmplifyAnimationPack/Blueprints/Character/BP_Character.charAnimCommunicator` player))
  (bind (_returnvalue_x_2 _returnvalue_y_2) (`KismetMathLibrary.BreakVector` (`KismetMathLibrary.GetDirectionUnitVector` _returnvalue (`self.K2_GetActorLocation`))))
  (`/Game/AmplifyAnimationPack/Blueprints/Character/BP_Character.UI_HideInteractionUI` player)
  (`/Game/AmplifyAnimationPack/Blueprints/Character/BP_Character.ChangeCurrentState` player "/Game/AmplifyAnimationPack/Blueprints/Character/CharacterStates/BP_InteractionState.BP_InteractionState_C")
  (if (not (`KismetMathLibrary.ClassIsChildOf` (`GameplayStatics.GetObjectClass` self) "/Game/AmplifyAnimationPack/Blueprints/Weapons/BP_WeaponActor.BP_WeaponActor_C"))
    (set `/Game/AmplifyAnimationPack/Blueprints/Character/BP_Character.objectPickedUp` self player))
  (if (> _returnvalue_y_2 0.3)
    (`/Game/AmplifyAnimationPack/Animations/Character/Anim_Blueprints/Interfaces/BPI_AnimComunicator.Set_PickObjDirVal` _charanimcommunicator "NewEnumerator2")
    (elif (< _returnvalue_y_2 -0.3)
      (`/Game/AmplifyAnimationPack/Animations/Character/Anim_Blueprints/Interfaces/BPI_AnimComunicator.Set_PickObjDirVal` _charanimcommunicator "NewEnumerator1")
      (else
        (`/Game/AmplifyAnimationPack/Animations/Character/Anim_Blueprints/Interfaces/BPI_AnimComunicator.Set_PickObjDirVal` _charanimcommunicator "NewEnumerator0"))))
  (if (>= (`KismetMathLibrary.Abs` (- _returnvalue_z (.z _returnvalue))) 30.0)
    (`/Game/AmplifyAnimationPack/Animations/Character/Anim_Blueprints/Interfaces/BPI_AnimComunicator.Set_InteractionTypeVal` _charanimcommunicator "NewEnumerator1")
    (else
      (`/Game/AmplifyAnimationPack/Animations/Character/Anim_Blueprints/Interfaces/BPI_AnimComunicator.Set_InteractionTypeVal` _charanimcommunicator "NewEnumerator11"))))

(fn `CheckResetPlayerCrouch`
  (returns (willReset :type Boolean))
  (return true))

(fn `UserConstructionScript`)