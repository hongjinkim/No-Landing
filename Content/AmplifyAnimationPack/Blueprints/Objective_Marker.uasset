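; Objective marker actor that displays the player's distance to it through a widget component.
; Every Tick it measures the horizontal distance to the player character, ignoring height, converts it to truncated whole meters and passes it to the widget's UpdateTextMessage.
; The construction script sets a vector parameter on the Marker's materials, but the parameter name is None.
; The overlap event is an empty stub.
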(event `self.ReceiveTick`
  (params (DeltaSeconds :type "Float (single-precision)"))
  (message `/Game/AmplifyAnimationPack/Blueprints/Widgets/BPI_Marker_Widget.UpdateText` (`WidgetComponent.GetUserWidgetObject` (`self.marker widget`)) (`KismetTextLibrary.Conv_DoubleToText` (`KismetMathLibrary.Conv_IntToDouble` (`KismetMathLibrary.FTrunc` (/ (`KismetMathLibrary.Vector_Distance` (`KismetMathLibrary.MakeVector` (.x (`self.K2_GetActorLocation`)) (.y (`self.K2_GetActorLocation`))) (`KismetMathLibrary.MakeVector` (.x (`self.K2_GetActorLocation` (`GameplayStatics.GetPlayerCharacter` 0))) (.y (`self.K2_GetActorLocation` (`GameplayStatics.GetPlayerCharacter` 0))))) 100.0))) "HalfToEven")))

(fn `UserConstructionScript`
  (`MeshComponent.SetVectorParameterValueOnMaterials` (`self.Marker`) "None" (0.0 0.0 0.0)))