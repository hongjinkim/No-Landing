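; Light source Blueprint whose brightness follows the DopingTime value of a referenced CastBP object.
; Every Tick it sets its LightComponent intensity to that value plus a base of one.
; A branch that would switch the color between white and red-orange based on DopingTime is disconnected and never runs.
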(event `self.ReceiveTick`
  (params (DeltaSeconds :type "Float (single-precision)"))
  ;[1 1 1] light
  (`LightComponent.SetIntensity` (`self.LightComponent`) (+ (* (`/Game/AmplifyAnimationPack/Blueprints/Character/BP_Character.DopingTime` (`self.Cast_BP`)) 1.0) 1.0)))

(fn `UserConstructionScript`)