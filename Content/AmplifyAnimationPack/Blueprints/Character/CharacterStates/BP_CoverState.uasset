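; Character state for taking cover against a wall, standing or crouched, in the Amplify Animation Pack.
; Input handlers use the character's cover traces to choose moving, edge sneaking, corner turns, stance changes, exiting, and shooting, aiming or throwing from either side or over the top.
; Choices go to CharAnimCommunicator as animation values, with CanMove gating input during actions.
; Each update offsets the camera, aligns to the wall normal and checks whether low cover requires crouching.
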(fn `Camera_UpdateOffset`
  (params (deltaTime :type "Float (double-precision)"))
  (bind _deltatime (`local.deltaTime`))
  (bind _charanimcommunicator (`/Game/AmplifyAnimationPack/Blueprints/Character/BP_Character.charAnimCommunicator` (`self.charRef`)))
  (bind _cameraarm (`/Game/AmplifyAnimationPack/Blueprints/Character/BP_Character.CameraArm` (`self.charRef`)))
  (bind (_socketoffset_x _socketoffset_y _socketoffset_z) (`KismetMathLibrary.BreakVector` (`SpringArmComponent.SocketOffset` _cameraarm)))
  (if (`self.isInEntry`)
    (return)
    (else
      (bind _curentvalue (`/Game/AmplifyAnimationPack/Animations/Character/Anim_Blueprints/Interfaces/BPI_AnimComunicator.Get_CoverActionVal` _charanimcommunicator))
      (bind _curentvalue_2 (`/Game/AmplifyAnimationPack/Animations/Character/Anim_Blueprints/Interfaces/BPI_AnimComunicator.Get_CoverDirVal` _charanimcommunicator))
      (set `SpringArmComponent.SocketOffset` (`KismetMathLibrary.MakeVector` (`KismetMathLibrary.FInterpTo` _socketoffset_x -30.0 _deltatime 7.0) (`KismetMathLibrary.FInterpTo` _socketoffset_y (* (select `/Game/AmplifyAnimationPack/Blueprints/Character/CharacterEnumerators/Character_CoverFacingDir_Enum` _curentvalue_2 :`NewEnumerator1` 1.0 :`NewEnumerator0` (`KismetMathLibrary.SelectFloat` 1.0 -1.0 (`|EnumEquality` _curentvalue "NewEnumerator9"))) (select `/Game/AmplifyAnimationPack/Blueprints/Character/CharacterEnumerators/Character_CoverActions_Enum` _curentvalue :`NewEnumerator0` 50.0 :`NewEnumerator1` 70.0 :`NewEnumerator2` 150.0 :`NewEnumerator5` 150.0 :`NewEnumerator7` 50.0 :`NewEnumerator10` 55.0 :`NewEnumerator9` 55.0 :!type "Float (single-precision)")) _deltatime 3.5) _socketoffset_z) _cameraarm))))

(fn `Cover_DecideAttack`
  (params (willForceUp :type Boolean))
  (bind _charref (`self.charRef`))
  (bind _charref_2 (`self.charRef`))
  (`/Game/AmplifyAnimationPack/Animations/Character/Anim_Blueprints/Interfaces/BPI_AnimComunicator.Set_IsAimCoverUpVal` (`/Game/AmplifyAnimationPack/Blueprints/Character/BP_Character.charAnimCommunicator` _charref) willForceUp)
  (if (`KismetSystemLibrary.IsValid` (`/Game/AmplifyAnimationPack/Blueprints/Character/BP_Character.currentWeapon` _charref))
    (`/Game/AmplifyAnimationPack/Blueprints/Character/BP_Character.Weapon_StartShooting` _charref_2)
    (else
      (`/Game/AmplifyAnimationPack/Animations/Character/Anim_Blueprints/Interfaces/BPI_AnimComunicator.Set_CoverActionVal` (`/Game/AmplifyAnimationPack/Blueprints/Character/BP_Character.charAnimCommunicator` _charref_2) "NewEnumerator5"))))

(fn `Cover_DetectCanTriggerAttack`
  (returns (canTrigger :type Boolean) (willBeUp :type Boolean))
  (bind _charref (`self.charRef`))
  (bind _charref_2 (`self.charRef`))
  (bind _charref_3 (`self.charRef`))
  (bind _charanimcommunicator (`/Game/AmplifyAnimationPack/Blueprints/Character/BP_Character.charAnimCommunicator` _charref))
  (bind _curentvalue (`/Game/AmplifyAnimationPack/Animations/Character/Anim_Blueprints/Interfaces/BPI_AnimComunicator.Get_WeaponActionVal` (`/Game/AmplifyAnimationPack/Blueprints/Character/BP_Character.charAnimCommunicator` _charref_3)))
  (if (or (and (`KismetSystemLibrary.IsValid` (`/Game/AmplifyAnimationPack/Blueprints/Character/BP_Character.currentWeapon` _charref_3)) (`|EnumInequality` _curentvalue "NewEnumerator5")) (`KismetSystemLibrary.IsValid` (`/Game/AmplifyAnimationPack/Blueprints/Character/BP_Character.objectPickedUp` _charref_3)))
    (bind _ishitting (`/Game/AmplifyAnimationPack/Blueprints/Character/BP_Character.Cover_LinetraceMovement` (`self.charRef`) -1.0))
    (if (not _ishitting)
      (set `self.canMove` false)
      (`/Game/AmplifyAnimationPack/Animations/Character/Anim_Blueprints/Interfaces/BPI_AnimComunicator.Set_CoverDirVal` (`/Game/AmplifyAnimationPack/Blueprints/Character/BP_Character.charAnimCommunicator` _charref_2) "NewEnumerator0")
      (return true false)
      (else
        (bind _ishitting_2 (`/Game/AmplifyAnimationPack/Blueprints/Character/BP_Character.Cover_LinetraceMovement` _charref_2 1.0))
        (if (not _ishitting_2)
          (set `self.canMove` false)
          (`/Game/AmplifyAnimationPack/Animations/Character/Anim_Blueprints/Interfaces/BPI_AnimComunicator.Set_CoverDirVal` _charanimcommunicator "NewEnumerator1")
          (return true false)
          (else
            (bind _curentvalue_2 (`/Game/AmplifyAnimationPack/Animations/Character/Anim_Blueprints/Interfaces/BPI_AnimComunicator.Get_MovementStateVal` _charanimcommunicator))
            (bind _ishitting_3 (`/Game/AmplifyAnimationPack/Blueprints/Character/BP_Character.Cover_LinetraceCheckCrouchUp` _charref 0.0 -1.0))
            (if (and (not _ishitting_3) (`|EnumEquality` _curentvalue_2 "NewEnumerator19"))
              (set `self.canMove` false)
              (return true true)
              (else
                (return false false)))))))
    (else
      (return false false))))

(fn `Cover_ForceCrouch`
  (bind _charref (`self.charRef`))
  (bind _charanimcommunicator (`/Game/AmplifyAnimationPack/Blueprints/Character/BP_Character.charAnimCommunicator` (`self.charRef`)))
  (bind _curentvalue (`/Game/AmplifyAnimationPack/Animations/Character/Anim_Blueprints/Interfaces/BPI_AnimComunicator.Get_MovementStateVal` _charanimcommunicator))
  (if (`|EnumInequality` _curentvalue "NewEnumerator19")
    (`/Game/AmplifyAnimationPack/Animations/Character/Anim_Blueprints/Interfaces/BPI_AnimComunicator.Set_MovementStateVal` _charanimcommunicator "NewEnumerator19")
    (`/Game/AmplifyAnimationPack/Blueprints/Character/BP_Character.Crouch_AdjustCharacter` _charref true (`Actor.K2_GetActorLocation` _charref))))

(fn `Cover_StartAiming`
  (params (willForceUp :type Boolean))
  (bind _charref (`self.charRef`))
  (bind _charref_2 (`self.CharRef`))
  (bind _charanimcommunicator (`/Game/AmplifyAnimationPack/Blueprints/Character/BP_Character.charAnimCommunicator` _charref_2))
  (bind _charanimcommunicator_2 (`/Game/AmplifyAnimationPack/Blueprints/Character/BP_Character.charAnimCommunicator` _charref))
  (bind _currentvalue (`/Game/AmplifyAnimationPack/Animations/Character/Anim_Blueprints/Interfaces/BPI_AnimComunicator.Set_IsAimCoverUpVal` _charanimcommunicator willForceUp))
  (`/Game/AmplifyAnimationPack/Animations/Character/Anim_Blueprints/Interfaces/BPI_AnimComunicator.Set_CoverActionVal` _charanimcommunicator "NewEnumerator10")
  (`/Game/AmplifyAnimationPack/Animations/Character/Anim_Blueprints/Interfaces/BPI_AnimComunicator.Set_UncoveredInitPosVal` _charanimcommunicator (`Actor.K2_GetActorLocation` _charref_2))
  (if _currentvalue
    (bind _forcegetup (`/Game/AmplifyAnimationPack/Blueprints/Character/BP_Character.Cover_LinetraceDetectAimHeight` _charref))
    (`/Game/AmplifyAnimationPack/Animations/Character/Anim_Blueprints/Interfaces/BPI_AnimComunicator.Set_ForceAimGetUpVal` _charanimcommunicator_2 _forcegetup)
    (else
      (`/Game/AmplifyAnimationPack/Animations/Character/Anim_Blueprints/Interfaces/BPI_AnimComunicator.Set_ForceAimGetUpVal` _charanimcommunicator_2 false))))

(fn `EnterState`
  (params (prevStateClass :type "/Game/AmplifyAnimationPack/Blueprints/Character/CharacterStates/BP_CharacterStateBase Class Reference"))
  (bind _charref (`self.charRef`))
  (bind _charref_2 (`self.charRef`))
  (bind _charref_3 (`self.charRef`))
  (bind _charactermovement (`Character.CharacterMovement` _charref))
  (bind _charanimcommunicator (`/Game/AmplifyAnimationPack/Blueprints/Character/BP_Character.charAnimCommunicator` (`self.charRef`)))
  (bind _charanimcommunicator_2 (`/Game/AmplifyAnimationPack/Blueprints/Character/BP_Character.charAnimCommunicator` (`self.charRef`)))
  (bind _charanimcommunicator_3 (`/Game/AmplifyAnimationPack/Blueprints/Character/BP_Character.charAnimCommunicator` _charref))
  (`parent.EnterState` null)
  (`MovementComponent.StopMovementImmediately` _charactermovement)
  (set `/Game/AmplifyAnimationPack/Blueprints/Character/BP_Character.canCrouchTransition` true _charref)
  (set `CharacterMovementComponent.bOrientRotationToMovement` false _charactermovement)
  (`/Game/AmplifyAnimationPack/Blueprints/Character/BP_Character.AdjustRotation` _charref (* (`/Game/AmplifyAnimationPack/Blueprints/Character/BP_Character.objToInteractRotVector` _charref) -1.0) false 0.0)
  (bind _ishitting (`/Game/AmplifyAnimationPack/Blueprints/Character/BP_Character.Cover_LinetraceCheckCrouchUp` (`self.charRef`) 0.0 1.0))
  (bind _curentvalue (`/Game/AmplifyAnimationPack/Animations/Character/Anim_Blueprints/Interfaces/BPI_AnimComunicator.Get_MovementStateVal` _charanimcommunicator_3))
  (bind _returnvalue (select `bool` _ishitting :`false` "NewEnumerator6" :`true` "NewEnumerator5" :!type "/Game/AmplifyAnimationPack/Blueprints/Character/CharacterEnumerators/Character_CoverTransitionTypes_Enum Enum"))
  (bind _currentvalue (`/Game/AmplifyAnimationPack/Animations/Character/Anim_Blueprints/Interfaces/BPI_AnimComunicator.Set_CoverTransitionVal` _charanimcommunicator_3 (select `/Game/AmplifyAnimationPack/Blueprints/Character/CharacterEnumerators/Character_MovementTypes_Enum` _curentvalue :`NewEnumerator0` _returnvalue :`NewEnumerator1` _returnvalue :`NewEnumerator2` "NewEnumerator7" :`NewEnumerator12` "NewEnumerator7" :`NewEnumerator13` "NewEnumerator7" :`NewEnumerator3` "NewEnumerator5" :`NewEnumerator7` "NewEnumerator5" :`NewEnumerator9` "NewEnumerator5" :`NewEnumerator10` "NewEnumerator5" :`NewEnumerator11` "NewEnumerator5" :`NewEnumerator8` "NewEnumerator5" :`NewEnumerator14` "NewEnumerator5" :`NewEnumerator16` "NewEnumerator5" :`NewEnumerator17` "NewEnumerator5" :`NewEnumerator18` "NewEnumerator5" :`NewEnumerator19` "NewEnumerator7" :`NewEnumerator20` "NewEnumerator5" :`NewEnumerator21` "NewEnumerator5" :`NewEnumerator22` "NewEnumerator5" :`NewEnumerator23` _returnvalue :`NewEnumerator24` "NewEnumerator5" :`NewEnumerator26` "NewEnumerator5" :`NewEnumerator25` "NewEnumerator5" :`NewEnumerator27` "NewEnumerator5" :`NewEnumerator4` "NewEnumerator5")))
  (`/Game/AmplifyAnimationPack/Animations/Character/Anim_Blueprints/Interfaces/BPI_AnimComunicator.Set_MovementStateVal` _charanimcommunicator (select `/Game/AmplifyAnimationPack/Blueprints/Character/CharacterEnumerators/Character_CoverTransitionTypes_Enum` _currentvalue :`NewEnumerator5` "NewEnumerator18" :`NewEnumerator6` "NewEnumerator19" :`NewEnumerator7` "NewEnumerator19" :`NewEnumerator8` "NewEnumerator0" :!type "/Game/AmplifyAnimationPack/Blueprints/Character/CharacterEnumerators/Character_MovementTypes_Enum Enum"))
  (`/Game/AmplifyAnimationPack/Animations/Character/Anim_Blueprints/Interfaces/BPI_AnimComunicator.Set_CoverActionVal` _charanimcommunicator "NewEnumerator0")
  (`/Game/AmplifyAnimationPack/Animations/Character/Anim_Blueprints/Interfaces/BPI_AnimComunicator.Set_CoverDirVal` _charanimcommunicator "NewEnumerator0")
  (`/Game/AmplifyAnimationPack/Blueprints/Character/BP_Character.SetNewCapsuleRadius` _charref_2 22.0 0.0)
  (`/Game/AmplifyAnimationPack/Blueprints/Character/BP_Character.AdjustPosition` _charref_2 (`Actor.K2_GetActorLocation` _charref_2) (* (`Actor.GetActorForwardVector` _charref_2) 30.0) true true false)
  (bind _asbp_cover_actor (cast `/Game/AmplifyAnimationPack/Blueprints/Interactables/BP_CoverActor` (`/Game/AmplifyAnimationPack/Blueprints/Character/BP_Character.objectToInteract` (`self.charRef`))))
  (set `self.currentWall` _asbp_cover_actor)
  (set `self.canMove` false)
  (`/Game/AmplifyAnimationPack/Animations/Character/Anim_Blueprints/Interfaces/BPI_AnimComunicator.Set_InputRightVal` _charanimcommunicator_2 0.0)
  (`/Game/AmplifyAnimationPack/Animations/Character/Anim_Blueprints/Interfaces/BPI_AnimComunicator.Set_InputFwdVal` _charanimcommunicator_2 0.0)
  (`/Game/AmplifyAnimationPack/Animations/Character/Anim_Blueprints/Interfaces/BPI_AnimComunicator.Set_SpeedVal` _charanimcommunicator_2 0.0)
  (bind _curentvalue_2 (`/Game/AmplifyAnimationPack/Animations/Character/Anim_Blueprints/Interfaces/BPI_AnimComunicator.Get_MovementStateVal` _charanimcommunicator_2))
  (bind _returnvalue_2 (`|EnumEquality` _curentvalue_2 "NewEnumerator19"))
  (set `self.mustBeCrouch` _returnvalue_2)
  (bind _curentvalue_3 (`/Game/AmplifyAnimationPack/Animations/Character/Anim_Blueprints/Interfaces/BPI_AnimComunicator.Get_CoverTransitionVal` _charanimcommunicator_2))
  (if (and _returnvalue_2 (`|EnumEquality` _curentvalue_3 "NewEnumerator6"))
    (`/Game/AmplifyAnimationPack/Blueprints/Character/BP_Character.Crouch_AdjustCharacter` _charref_3 true (`Actor.K2_GetActorLocation` _charref_3))))

(fn `Input_CrouchHold`
  (params (inputVal :type "Float (double-precision)"))
  (locals (newCoverState :type "/Game/AmplifyAnimationPack/Blueprints/Character/CharacterEnumerators/Character_MovementTypes_Enum Enum") (oldCoverState :type "/Game/AmplifyAnimationPack/Blueprints/Character/CharacterEnumerators/Character_MovementTypes_Enum Enum"))
  (bind _charref (`self.charRef`))
  (bind _charref_2 (`self.charRef`))
  (bind _charanimcommunicator (`/Game/AmplifyAnimationPack/Blueprints/Character/BP_Character.charAnimCommunicator` _charref_2))
  (bind _charanimcommunicator_2 (`/Game/AmplifyAnimationPack/Blueprints/Character/BP_Character.charAnimCommunicator` _charref))
  (`parent.Input_CrouchHold` 0.0)
  (if (not (`/Game/AmplifyAnimationPack/Blueprints/Character/BP_Character.isCrouchToggle` (`self.charRef`)))
    (bind _output_get (set `self.coverCrouchInput` (!= (`local.inputVal`) 0.0)))
    (if (and (`self.canMove`) (`/Game/AmplifyAnimationPack/Blueprints/Character/BP_Character.canCrouchTransition` _charref))
      (if (`self.mustBeCrouch`)
        (`self.Cover_ForceCrouch`)
        (else
          (bind _curentvalue (`/Game/AmplifyAnimationPack/Animations/Character/Anim_Blueprints/Interfaces/BPI_AnimComunicator.Get_MovementStateVal` _charanimcommunicator_2))
          (set `local.oldCoverState` _curentvalue)
          (bind _returnvalue (select `bool` _output_get :`false` "NewEnumerator18" :`true` "NewEnumerator19" :!type "/Game/AmplifyAnimationPack/Blueprints/Character/CharacterEnumerators/Character_MovementTypes_Enum Enum"))
          (bind _currentvalue (`/Game/AmplifyAnimationPack/Animations/Character/Anim_Blueprints/Interfaces/BPI_AnimComunicator.Set_MovementStateVal` _charanimcommunicator_2 _returnvalue))
          (set `local.newCoverState` _returnvalue)
          (if (`|EnumInequality` (`local.newCoverState`) (`local.oldCoverState`))
            (`/Game/AmplifyAnimationPack/Blueprints/Character/BP_Character.Crouch_AdjustCharacter` _charref_2 (`|EnumEquality` _currentvalue "NewEnumerator19") (`Actor.K2_GetActorLocation` _charref_2))
            (bind _curentvalue_2 (`/Game/AmplifyAnimationPack/Animations/Character/Anim_Blueprints/Interfaces/BPI_AnimComunicator.Get_InputRightVal` _charanimcommunicator))
            (if (== _curentvalue_2 0.0)
              (`/Game/AmplifyAnimationPack/Animations/Character/Anim_Blueprints/Interfaces/BPI_AnimComunicator.Set_CoverActionVal` _charanimcommunicator "NewEnumerator7")
              (set `self.canMove` false)))))
      (else
        (return)))))

(fn `Input_CrouchToggle`
  (locals (newCoverState :type "/Game/AmplifyAnimationPack/Blueprints/Character/CharacterEnumerators/Character_MovementTypes_Enum Enum") (oldCoverState :type "/Game/AmplifyAnimationPack/Blueprints/Character/CharacterEnumerators/Character_MovementTypes_Enum Enum"))
  (bind _charref (`self.charRef`))
  (bind _charref_2 (`self.charRef`))
  (bind _charref_3 (`self.charRef`))
  (bind _charanimcommunicator (`/Game/AmplifyAnimationPack/Blueprints/Character/BP_Character.charAnimCommunicator` _charref_2))
  (bind _charanimcommunicator_2 (`/Game/AmplifyAnimationPack/Blueprints/Character/BP_Character.charAnimCommunicator` _charref))
  (`parent.Input_CrouchToggle`)
  (if (`/Game/AmplifyAnimationPack/Blueprints/Character/BP_Character.isCrouchToggle` _charref_3)
    (bind _curentvalue (`/Game/AmplifyAnimationPack/Animations/Character/Anim_Blueprints/Interfaces/BPI_AnimComunicator.Get_MovementStateVal` (`/Game/AmplifyAnimationPack/Blueprints/Character/BP_Character.charAnimCommunicator` _charref_3)))
    (bind _output_get (set `self.coverCrouchInput` (`|EnumEquality` _curentvalue "NewEnumerator18")))
    (if (and (`self.canMove`) (`/Game/AmplifyAnimationPack/Blueprints/Character/BP_Character.canCrouchTransition` _charref))
      (if (`self.mustBeCrouch`)
        (`self.Cover_ForceCrouch`)
        (else
          (bind _curentvalue_2 (`/Game/AmplifyAnimationPack/Animations/Character/Anim_Blueprints/Interfaces/BPI_AnimComunicator.Get_MovementStateVal` _charanimcommunicator_2))
          (set `local.oldCoverState` _curentvalue_2)
          (bind _returnvalue (select `bool` _output_get :`false` "NewEnumerator18" :`true` "NewEnumerator19" :!type "/Game/AmplifyAnimationPack/Blueprints/Character/CharacterEnumerators/Character_MovementTypes_Enum Enum"))
          (bind _currentvalue (`/Game/AmplifyAnimationPack/Animations/Character/Anim_Blueprints/Interfaces/BPI_AnimComunicator.Set_MovementStateVal` _charanimcommunicator_2 _returnvalue))
          (set `local.newCoverState` _returnvalue)
          (if (`|EnumInequality` (`local.newCoverState`) (`local.oldCoverState`))
            (`/Game/AmplifyAnimationPack/Blueprints/Character/BP_Character.Crouch_AdjustCharacter` _charref_2 (`|EnumEquality` _currentvalue "NewEnumerator19") (`Actor.K2_GetActorLocation` _charref_2))
            (bind _curentvalue_3 (`/Game/AmplifyAnimationPack/Animations/Character/Anim_Blueprints/Interfaces/BPI_AnimComunicator.Get_InputRightVal` _charanimcommunicator))
            (if (== _curentvalue_3 0.0)
              (`/Game/AmplifyAnimationPack/Animations/Character/Anim_Blueprints/Interfaces/BPI_AnimComunicator.Set_CoverActionVal` _charanimcommunicator "NewEnumerator7")
              (set `self.canMove` false)))))
      (else
        (return)))
    (else
      (return))))

(fn `Input_Interact`
  (bind _charref (`self.charRef`))
  (bind _charanimcommunicator (`/Game/AmplifyAnimationPack/Blueprints/Character/BP_Character.charAnimCommunicator` (`self.charRef`)))
  (bind _charanimcommunicator_2 (`/Game/AmplifyAnimationPack/Blueprints/Character/BP_Character.charAnimCommunicator` (`self.charRef`)))
  (`parent.Input_Interact`)
  (bind _curentvalue (`/Game/AmplifyAnimationPack/Animations/Character/Anim_Blueprints/Interfaces/BPI_AnimComunicator.Get_CoverActionVal` _charanimcommunicator))
  (if (and (`self.canMove`) (`|EnumInequality` _curentvalue "NewEnumerator2") (`|EnumInequality` _curentvalue "NewEnumerator6"))
    (if (not (`self.coverCrouchInput`))
      (bind _curentvalue_2 (`/Game/AmplifyAnimationPack/Animations/Character/Anim_Blueprints/Interfaces/BPI_AnimComunicator.Get_MovementStateVal` _charanimcommunicator))
      (`/Game/AmplifyAnimationPack/Animations/Character/Anim_Blueprints/Interfaces/BPI_AnimComunicator.Set_CoverTransitionVal` _charanimcommunicator_2 (select `bool` (or (`|EnumEquality` _curentvalue_2 "NewEnumerator19") (`self.mustBeCrouch`)) :`false` "NewEnumerator5" :`true` "NewEnumerator8" :!type "/Game/AmplifyAnimationPack/Blueprints/Character/CharacterEnumerators/Character_CoverTransitionTypes_Enum Enum"))
      (else
        (`/Game/AmplifyAnimationPack/Animations/Character/Anim_Blueprints/Interfaces/BPI_AnimComunicator.Set_CoverTransitionVal` _charanimcommunicator_2 "NewEnumerator7")
        (`/Game/AmplifyAnimationPack/Animations/Character/Anim_Blueprints/Interfaces/BPI_AnimComunicator.Set_MovementStateVal` _charanimcommunicator_2 "NewEnumerator2")
        (`/Game/AmplifyAnimationPack/Animations/Character/Anim_Blueprints/Interfaces/BPI_AnimComunicator.Set_MovementStateVal` _charanimcommunicator_2 "NewEnumerator2")))
    (bind _curentvalue_3 (`/Game/AmplifyAnimationPack/Animations/Character/Anim_Blueprints/Interfaces/BPI_AnimComunicator.Get_CoverTransitionVal` _charanimcommunicator_2))
    (if (`|EnumEquality` _curentvalue_3 "NewEnumerator8")
      (`/Game/AmplifyAnimationPack/Blueprints/Character/BP_Character.Crouch_AdjustCharacter` _charref false (`Actor.K2_GetActorLocation` _charref)))
    (set `self.canMove` false)
    (`/Game/AmplifyAnimationPack/Animations/Character/Anim_Blueprints/Interfaces/BPI_AnimComunicator.Set_CoverActionVal` (`/Game/AmplifyAnimationPack/Blueprints/Character/BP_Character.charAnimCommunicator` (`self.charRef`)) "NewEnumerator9")
    (else
      (return))))

(fn `Input_Jump`
  (bind _charanimcommunicator (`/Game/AmplifyAnimationPack/Blueprints/Character/BP_Character.charAnimCommunicator` (`self.charRef`)))
  (`parent.Input_Jump`)
  (bind _curentvalue (`/Game/AmplifyAnimationPack/Animations/Character/Anim_Blueprints/Interfaces/BPI_AnimComunicator.Get_CoverActionVal` _charanimcommunicator))
  (if (`|EnumEquality` _curentvalue "NewEnumerator2")
    (bind _curentvalue_2 (`/Game/AmplifyAnimationPack/Animations/Character/Anim_Blueprints/Interfaces/BPI_AnimComunicator.Get_InputRightVal` _charanimcommunicator))
    (bind _ishitting (`/Game/AmplifyAnimationPack/Blueprints/Character/BP_Character.Cover_LinetraceCorner` (`self.charRef`) _curentvalue_2 -1.0))
    (if _ishitting
      (set `self.canMove` false)
      (`/Game/AmplifyAnimationPack/Animations/Character/Anim_Blueprints/Interfaces/BPI_AnimComunicator.Set_CoverActionVal` _charanimcommunicator "NewEnumerator3"))))

(fn `Input_MoveForward`
  (params (inputVal :type "Float (double-precision)"))
  (bind _charanimcommunicator (`/Game/AmplifyAnimationPack/Blueprints/Character/BP_Character.charAnimCommunicator` (`self.charRef`)))
  (`parent.Input_MoveForward` 0.0)
  (if (`self.canMove`)
    (bind _curentvalue (`/Game/AmplifyAnimationPack/Animations/Character/Anim_Blueprints/Interfaces/BPI_AnimComunicator.Get_MovementStateVal` (`/Game/AmplifyAnimationPack/Blueprints/Character/BP_Character.charAnimCommunicator` (`self.charRef`))))
    (if (and (`|EnumEquality` _curentvalue "NewEnumerator19") (> inputVal 0.0))
      (bind _ishitting (`/Game/AmplifyAnimationPack/Blueprints/Character/BP_Character.Cover_LinetraceCheckCrouchUp` (`self.charRef`) 0.0 -1.0))
      (if (not _ishitting)
        (`/Game/AmplifyAnimationPack/Animations/Character/Anim_Blueprints/Interfaces/BPI_AnimComunicator.Set_CoverActionVal` _charanimcommunicator "NewEnumerator6")
        (else
          (`/Game/AmplifyAnimationPack/Animations/Character/Anim_Blueprints/Interfaces/BPI_AnimComunicator.Set_CoverActionVal` _charanimcommunicator "NewEnumerator0")))
      (else
        (return)))
    (else
      (return))))

(fn `Input_MoveRight`
  (params (inputVal :type "Float (double-precision)"))
  (bind _charref (`self.charRef`))
  (bind _charref_2 (`self.charRef`))
  (bind _charref_3 (`self.charRef`))
  (bind _charanimcommunicator (`/Game/AmplifyAnimationPack/Blueprints/Character/BP_Character.charAnimCommunicator` _charref))
  (bind _charanimcommunicator_2 (`/Game/AmplifyAnimationPack/Blueprints/Character/BP_Character.charAnimCommunicator` _charref_2))
  (`parent.Input_MoveRight` 0.0)
  (if (`self.canMove`)
    (bind _output_get (set `/Game/AmplifyAnimationPack/Blueprints/Character/BP_Character.InputRight` inputVal _charref))
    (bind _currentval (`/Game/AmplifyAnimationPack/Animations/Character/Anim_Blueprints/Interfaces/BPI_AnimComunicator.Set_InputRightVal` _charanimcommunicator _output_get))
    (if (!= _currentval 0.0)
      (bind _ishitting (`/Game/AmplifyAnimationPack/Blueprints/Character/BP_Character.Cover_LinetraceCorner` _charref inputVal 1.0))
      (if _ishitting
        (`/Game/AmplifyAnimationPack/Animations/Character/Anim_Blueprints/Interfaces/BPI_AnimComunicator.Set_CoverActionVal` (`/Game/AmplifyAnimationPack/Blueprints/Character/BP_Character.charAnimCommunicator` _charref_3) "NewEnumerator4")
        (set `self.canMove` false)
        (else
          (bind (_ishitting_2 _collidingactor) (`/Game/AmplifyAnimationPack/Blueprints/Character/BP_Character.Cover_LinetraceMovement` _charref_3 inputVal))
          (if (and _ishitting_2 (== _collidingactor (`self.currentWall`)))
            (`/Game/AmplifyAnimationPack/Animations/Character/Anim_Blueprints/Interfaces/BPI_AnimComunicator.Set_CoverActionVal` _charanimcommunicator_2 "NewEnumerator1")
            (else
              (`/Game/AmplifyAnimationPack/Animations/Character/Anim_Blueprints/Interfaces/BPI_AnimComunicator.Set_CoverActionVal` _charanimcommunicator_2 "NewEnumerator2")
              (`MovementComponent.StopMovementImmediately` (`Character.CharacterMovement` _charref_2))))))
      (else
        (`/Game/AmplifyAnimationPack/Animations/Character/Anim_Blueprints/Interfaces/BPI_AnimComunicator.Set_CoverActionVal` _charanimcommunicator "NewEnumerator0")))
    (else
      (return))))

(fn `Input_WeaponAim`
  (`parent.Input_WeaponAim`)
  (bind _curentvalue (`/Game/AmplifyAnimationPack/Animations/Character/Anim_Blueprints/Interfaces/BPI_AnimComunicator.Get_IsUncoveredVal` (`/Game/AmplifyAnimationPack/Blueprints/Character/BP_Character.charAnimCommunicator` (`self.charRef`))))
  (if (and (`self.CanExecuteWeaponAction`) (not _curentvalue))
    (bind (_cantrigger _willbeup) (`self.Cover_DetectCanTriggerAttack`))
    (if _cantrigger
      (`self.Cover_StartAiming` _willbeup))))

(fn `Input_WeaponAim_Released`
  (`parent.Input_WeaponAim_Released`)
  (bind _curentvalue (`/Game/AmplifyAnimationPack/Animations/Character/Anim_Blueprints/Interfaces/BPI_AnimComunicator.Get_CoverActionVal` (`/Game/AmplifyAnimationPack/Blueprints/Character/BP_Character.charAnimCommunicator` (`self.charRef`))))
  (if (`|EnumEquality` _curentvalue "NewEnumerator10")
    (`/Game/AmplifyAnimationPack/Animations/Character/Anim_Blueprints/Interfaces/BPI_AnimComunicator.Set_CoverActionVal` (`/Game/AmplifyAnimationPack/Blueprints/Character/BP_Character.charAnimCommunicator` (`self.charRef`)) "NewEnumerator0")
    (set `self.canMove` true)))

(fn `Input_WeaponEquip`
  (`parent.Input_WeaponEquip`)
  (if (`self.canMove`)
    (`/Game/AmplifyAnimationPack/Blueprints/Character/BP_Character.Weapon_ChangeWeapon` (`self.charRef`))))

(fn `Input_WeaponReload`
  (`parent.Input_WeaponReload`)
  (if (`self.CanExecuteWeaponAction`)
    (`/Game/AmplifyAnimationPack/Blueprints/Character/BP_Character.Weapon_Reload` (`self.charRef`))))

(fn `Input_WeaponShoot`
  (bind _charref (`self.charRef`))
  (`parent.Input_WeaponShoot`)
  (bind _curentvalue (`/Game/AmplifyAnimationPack/Animations/Character/Anim_Blueprints/Interfaces/BPI_AnimComunicator.Get_IsUncoveredVal` (`/Game/AmplifyAnimationPack/Blueprints/Character/BP_Character.charAnimCommunicator` _charref)))
  (if (or (`self.CanExecuteWeaponAction`) (and _curentvalue (`/Game/AmplifyAnimationPack/Blueprints/Character/BP_Character.Is Aiming` _charref)) (`KismetSystemLibrary.IsValid` (`/Game/AmplifyAnimationPack/Blueprints/Character/BP_Character.objectPickedUp` _charref)))
    (bind (_cantrigger _willbeup) (`self.Cover_DetectCanTriggerAttack`))
    (if _cantrigger
      (`self.Cover_DecideAttack` _willbeup))))

(fn `Input_WeaponShoot_Released`
  (bind _charref (`self.charRef`))
  (bind _charanimcommunicator (`/Game/AmplifyAnimationPack/Blueprints/Character/BP_Character.charAnimCommunicator` _charref))
  (bind _is_aiming (`/Game/AmplifyAnimationPack/Blueprints/Character/BP_Character.Is Aiming` _charref))
  (`parent.Input_WeaponShoot_Released`)
  (bind _curentvalue (`/Game/AmplifyAnimationPack/Animations/Character/Anim_Blueprints/Interfaces/BPI_AnimComunicator.Get_WeaponTypeVal` _charanimcommunicator))
  (bind _curentvalue_2 (`/Game/AmplifyAnimationPack/Animations/Character/Anim_Blueprints/Interfaces/BPI_AnimComunicator.Get_WeaponActionVal` _charanimcommunicator))
  (if (and (`|EnumInequality` _curentvalue "NewEnumerator0") (`|EnumEquality` _curentvalue_2 "NewEnumerator1"))
    (`/Game/AmplifyAnimationPack/Animations/Character/Anim_Blueprints/Interfaces/BPI_AnimComunicator.Set_WeaponActionVal` (`/Game/AmplifyAnimationPack/Blueprints/Character/BP_Character.charAnimCommunicator` (`self.charRef`)) (select `bool` _is_aiming :`false` "NewEnumerator0" :`true` "NewEnumerator3" :!type "/Game/AmplifyAnimationPack/Blueprints/Character/CharacterEnumerators/Character_WeaponAction_Enum Enum"))
    (set `self.canMove` (not _is_aiming))))

(fn `SetCharVelocityAnim`
  (bind _charref (`self.charRef`))
  (`/Game/AmplifyAnimationPack/Animations/Character/Anim_Blueprints/Interfaces/BPI_AnimComunicator.Set_CharVelocityVal` (`/Game/AmplifyAnimationPack/Blueprints/Character/BP_Character.charAnimCommunicator` _charref) (`KismetMathLibrary.VSize` (`Actor.GetVelocity` _charref))))

(fn `UpdateState`
  (params (deltaTime :type "Float (double-precision)"))
  (bind _charref (`self.charRef`))
  (bind _charref_2 (`self.charRef`))
  (`parent.UpdateState` 0.0)
  (`self.Camera_UpdateOffset` deltaTime)
  (bind _curentvalue (`/Game/AmplifyAnimationPack/Animations/Character/Anim_Blueprints/Interfaces/BPI_AnimComunicator.Get_IsUncoveredVal` (`/Game/AmplifyAnimationPack/Blueprints/Character/BP_Character.charAnimCommunicator` _charref)))
  (if (not _curentvalue)
    (bind _curentvalue_2 (`/Game/AmplifyAnimationPack/Animations/Character/Anim_Blueprints/Interfaces/BPI_AnimComunicator.Get_CoverDirVal` (`/Game/AmplifyAnimationPack/Blueprints/Character/BP_Character.charAnimCommunicator` _charref)))
    (bind _ishitting (`/Game/AmplifyAnimationPack/Blueprints/Character/BP_Character.Cover_LinetraceCheckCrouchUp` _charref (select `/Game/AmplifyAnimationPack/Blueprints/Character/CharacterEnumerators/Character_CoverFacingDir_Enum` _curentvalue_2 :`NewEnumerator1` -25.0 :`NewEnumerator0` 25.0 :!type "Float (single-precision)") -1.0))
    (set `self.mustBeCrouch` (not _ishitting)))
  (if (`self.canMove`)
    (bind (_ishitting_2 _hit) (`/Game/AmplifyAnimationPack/Blueprints/Character/BP_Character.Cover_LinetraceWall` _charref_2))
    (if _ishitting_2
      (bind (_bblockinghit _binitialoverlap _time _distance _location _impactpoint _normal _impactnormal _physmat _hitactor) (`GameplayStatics.BreakHitResult` _hit))
      (set `self.currentWall` _hitactor)
      (`/Game/AmplifyAnimationPack/Blueprints/Character/BP_Character.AdjustRotation` _charref_2 (`KismetMathLibrary.Conv_RotatorToVector` (`KismetMathLibrary.Conv_VectorToRotator` _normal)) true 7.0))
    (else
      (return))))

(fn `UpdateStateAnimation`
  (bind _charref (`self.charRef`))
  (`parent.UpdateStateAnimation`)
  (`self.SetCharVelocityAnim`)
  (if (and (`self.mustBeCrouch`) (`self.canMove`) (`/Game/AmplifyAnimationPack/Blueprints/Character/BP_Character.canCrouchTransition` _charref) (`/Game/AmplifyAnimationPack/Blueprints/Character/BP_Character.isCrouchToggle` _charref))
    (`self.Cover_ForceCrouch`)
    (else
      (return))))