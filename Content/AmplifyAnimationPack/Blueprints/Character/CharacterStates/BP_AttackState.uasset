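; BP_AttackState is the character state for attacking in the Amplify Animation Pack character's state machine.
; On entry it clears the combo flag and index through CharAnimCommunicator, and each update switches to BP_FallingState when the character moves downward without ground beneath.
; On exit it resets movement state, combat action and combo index if one specific movement state is still set.
; Attack input only calls the parent handler; its AttackStart call is disconnected.
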(fn `CheckIsGrounded`
  (bind _charref (`self.charRef`))
  (if (< (.z (`CharacterMovementComponent.GetLastUpdateVelocity` (`Character.CharacterMovement` _charref))) 0.0)
    (bind (_groundhitresult _isgrounded) (`/Game/AmplifyAnimationPack/Blueprints/Character/BP_Character.Ground_SpheretraceDetector` _charref))
    (if (not _isgrounded)
      (`/Game/AmplifyAnimationPack/Blueprints/Character/BP_Character.ChangeCurrentState` _charref "/Game/AmplifyAnimationPack/Blueprints/Character/CharacterStates/BP_FallingState.BP_FallingState_C"))))

(fn `EnterState`
  (params (prevStateClass :type "/Game/AmplifyAnimationPack/Blueprints/Character/CharacterStates/BP_CharacterStateBase Class Reference"))
  (bind _charanimcommunicator (`/Game/AmplifyAnimationPack/Blueprints/Character/BP_Character.charAnimCommunicator` (`self.charRef`)))
  (`parent.EnterState` null)
  (`/Game/AmplifyAnimationPack/Animations/Character/Anim_Blueprints/Interfaces/BPI_AnimComunicator.Set_CanComboAttackVal` _charanimcommunicator false)
  (`/Game/AmplifyAnimationPack/Animations/Character/Anim_Blueprints/Interfaces/BPI_AnimComunicator.Set_ComboAttackIndexVal` _charanimcommunicator 0))

(fn `ExitState`
  (bind _charanimcommunicator (`/Game/AmplifyAnimationPack/Blueprints/Character/BP_Character.charAnimCommunicator` (`self.charRef`)))
  (`parent.ExitState`)
  (bind _curentvalue (`/Game/AmplifyAnimationPack/Animations/Character/Anim_Blueprints/Interfaces/BPI_AnimComunicator.Get_MovementStateVal` _charanimcommunicator))
  (if (`|EnumEquality` _curentvalue "NewEnumerator4")
    (`/Game/AmplifyAnimationPack/Animations/Character/Anim_Blueprints/Interfaces/BPI_AnimComunicator.Set_MovementStateVal` _charanimcommunicator "NewEnumerator0")
    (`/Game/AmplifyAnimationPack/Animations/Character/Anim_Blueprints/Interfaces/BPI_AnimComunicator.Set_CombatActionVal` _charanimcommunicator "NewEnumerator0")
    (`/Game/AmplifyAnimationPack/Animations/Character/Anim_Blueprints/Interfaces/BPI_AnimComunicator.Set_ComboAttackIndexVal` _charanimcommunicator 0)))

(fn `Input_Attack`
  (params (AttackState :type "/Game/AmplifyAnimationPack/Blueprints/Character/CharacterEnumerators/Character_CombatAction_Enum Enum" :default "NewEnumerator0"))
  (`parent.Input_Attack` "NewEnumerator0"))

(fn `UpdateState`
  (params (deltaTime :type "Float (double-precision)"))
  (`parent.UpdateState` 0.0)
  (`self.CheckIsGrounded`))