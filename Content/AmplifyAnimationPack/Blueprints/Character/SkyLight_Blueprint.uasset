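; Sky light Blueprint that tints the scene's ambient light according to the player character's doping timer.
; Every Tick it casts the player pawn to BP_Character and compares DopingTime to a threshold just under ten.
; The light turns red at or below that threshold and blue above it, switching instantly with no blend.
; A SetIntensity call is left unconnected and never runs.
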(event `self.ReceiveTick`
  (params (DeltaSeconds :type "Float (single-precision)"))
  ;[1 1 1] light
  (`|ExecutionSequence`
    (:`then_0`
      (bind _asbp_character (cast `/Game/AmplifyAnimationPack/Blueprints/Character/BP_Character` (`GameplayStatics.GetPlayerPawn` 0))))
    (:`then_1`
      (if (<= (`/Game/AmplifyAnimationPack/Blueprints/Character/BP_Character.DopingTime` _asbp_character) 9.9)
        (`SkyLightComponent.SetLightColor` (`self.LightComponent`) (struct :`R` 0.854167 :`B` 0.029647 :`A` 1.0))
        (else
          (`SkyLightComponent.SetLightColor` (`self.LightComponent`) (struct :`G` 0.095591 :`B` 1.0 :`A` 1.0)))))))

(fn `UserConstructionScript`)