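; Enemy character that pursues the player and dies after taking enough hits.
; On BeginPlay it caches the player's BP_Character, starts an AIMoveTo chase that re-issues itself on success or failure, and sets Health from its default.
; OnHit subtracts Damage, prints the remaining health, and drives the player's crosshair hit fade, flagging a kill and destroying the enemy when health runs out.
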(event `self.ReceiveBeginPlay`
  (bind _asbp_character (cast `/Game/AmplifyAnimationPack/Blueprints/Character/BP_Character` (`GameplayStatics.GetPlayerCharacter` 0)))
  (bind _output_get (set `self.Char REF` _asbp_character))
  (`self.Chase Player` _output_get)
  (set `self.Health` (`self.Default Health`)))

(event `Chase Player`
  (params (PlayerToChase :type "/Game/AmplifyAnimationPack/Blueprints/Character/BP_Character Object Reference"))
  (`|AIMoveTo` self (0.0 0.0 0.0) PlayerToChase
    (:`OnSuccess`
      _)
    (:`OnFail`
      _))
  (`self.Chase Player` (`self.Char REF`)))

(fn `OnHit`
  (bind _crosshair (`/Game/AmplifyAnimationPack/Blueprints/Character/BP_Character.CrossHair` (`self.Char REF`)))
  (bind _output_get (set `self.Health` (- (`self.Health`) (`self.Damage`))))
  (`KismetSystemLibrary.PrintText` (`KismetTextLibrary.Conv_DoubleToText` _output_get "HalfToEven"))
  (if (<= _output_get 0.0)
    (set `/Game/AmplifyAnimationPack/Blueprints/Widgets/HUD/Crosshair.Killed Enemy` true _crosshair)
    (`self.K2_DestroyActor`))
  (`/Game/AmplifyAnimationPack/Blueprints/Widgets/HUD/Crosshair.OnHit_Fade_Out` _crosshair "Forward"))

(fn `UserConstructionScript`)