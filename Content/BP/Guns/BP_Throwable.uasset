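; BP_Throwable is a throwable actor with a grenade mesh that can be thrown once from an attached state.
; Throw detaches it and launches it with ProjectileMovement while the mesh rotates to a random orientation.
; After a short delay it enables collision and switches to physics simulation, carrying over its velocity, then sets a lifespan.
; The first root hit plays a sound and makes noise.
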(event `self.ReceiveBeginPlay`)

(event `/Game/BP/CLM_BPI_Throwable.Throw`
  (params (Velocity :type "Vector Structure"))
  (bind _root (`self.Root`))
  (bind _projectilemovement (`self.ProjectileMovement`))
  (`/Engine/EditorBlueprintResources/StandardMacros.DoOnce` false
    (:`Completed`
      (`|ExecutionSequence`
        (:`then_0`
          (`self.K2_DetachFromActor` "KeepWorld" "KeepWorld" "KeepWorld")
          (set `MovementComponent.Velocity` Velocity _projectilemovement)
          (`ActorComponent.Activate` _projectilemovement false)
          (`KismetSystemLibrary.Delay` 0.3)
          (`PrimitiveComponent.SetCollisionEnabled` (`self.Root`) "QueryAndPhysics")
          (bind _output_get (set `self.velocity` (`self.GetVelocity`)))
          (`PrimitiveComponent.SetSimulatePhysics` _root true)
          (`PrimitiveComponent.SetPhysicsLinearVelocity` _root _output_get false "None")
          (`KismetSystemLibrary.Delay` 1.0)
          (`self.SetLifeSpan` 3.0))
        (:`then_1`
          (`KismetSystemLibrary.MoveComponentTo` (`self.SM Grenade`) (0.0 0.0 0.0) (`KismetMathLibrary.RandomRotator` false) false false 0.5))))))

(event `self.Root.OnComponentHit`
  (params (HitComponent :type "PrimitiveComponent Object Reference") (OtherActor :type "Actor Object Reference") (OtherComp :type "PrimitiveComponent Object Reference") (NormalImpulse :type "Vector Structure") (Hit :type "HitResult Structure (by ref)"))
  (bind _returnvalue (`self.K2_GetActorLocation`))
  (`/Engine/EditorBlueprintResources/StandardMacros.DoOnce` false
    (:`Completed`
      (`self.MakeNoise` 1.0 null _returnvalue 0.0 "0")
      (`GameplayStatics.PlaySoundAtLocation` (`self.Hit sound`) _returnvalue (struct) 1.0 1.0 0.0 null null null))))

(fn `UserConstructionScript`
  (`PrimitiveComponent.SetCollisionEnabled` (`self.Root`) "NoCollision")
  (`PrimitiveComponent.SetAllMassScale` (`self.Root`) 0.4))