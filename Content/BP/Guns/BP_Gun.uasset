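; Generic gun actor that characters equip, fire, reload and drop, with an overlap prompt letting the player pick up or swap it.
; Fire loops shots for automatic weapons, checking ammo and auto-reloading with stance-based montages while driving recoil, reticle and ammo widget.
; Shots multi-trace toward the character's randomly deviated target, using a surface penetration map and spawning per-surface impacts, trails and noise.
; Character communication runs through message calls, with player-only UI.
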(event `self.ReceiveBeginPlay`
  (`/Engine/EditorBlueprintResources/StandardMacros.IsValid` (`self.GetParentActor`)
    (:`Is Not Valid`
      (`self.SetInteractable` true))))

(event `self.Fire`
  (params (`start/stop` :type Boolean))
  (bind _ch_shoot_standing (`self.ch_shoot_standing`))
  (bind _character (`self.character`))
  (bind _recoil_pitch_input (`self.recoil pitch input`))
  (bind _output_get (set `self.firing` `start/stop`))
  (if (not (`self.reloading`))
    (`self.Check Ammo`
      (:`then`
        _)
      (:`reloading`
        _))
    (`|PlayMontage` (`self.gun mesh`) (`self.gun_shoot_montage`) 1.0 0.0 (select `bool` _output_get :`false` "release" :`true` "Default" :!type "Name")
      (:`then`
        (message `/Game/BP/CLM_BPI_Character.PlayCharacterMontage` _character _ch_shoot_standing)
        (if _output_get :!label _label
          (`self.UpdateReticle` 0.2)
          (`self.Check Ammo`
            (:`then`
              _)
            (:`reloading`
              (message `/Game/BP/CLM_BPI_Character.PlayCharacterMontage` (`self.character`) (`self.ch_shoot_standing`))))
          (if (`self.firing`)
            (`ActorComponent.Activate` (`self.P_BulletShell`) true)
            (`ActorComponent.Activate` (`self.NS_flash`) false)
            (`GameplayStatics.PlaySoundAtLocation` (`self.shoot sound`) (`self.K2_GetActorLocation`) (struct) 2.0 1.0 0.0 null null null)
            (`self.Emit Bullet`)
            (`/Engine/EditorBlueprintResources/StandardMacros.DecrementInt` (`self.loaded ammo count`)
              (:`  `
                (`self.UpdateAmmoCount`)
                (message `/Game/BP/CLM_BPI_Character.AddRecoil` (`self.character`) (`self.recoil rotaiton`) _recoil_pitch_input)
                (set `self.recoil pitch input` (* _recoil_pitch_input 0.8))
                (`KismetSystemLibrary.Delay` (`self.bullet_delay`))
                (`ActorComponent.Deactivate` (`self.NS_flash`))
                (if (`self.automatic`)
                  (goto _label)))))
          (else
            (if (`self.automatic`)
              (message `/Game/BP/CLM_BPI_Character.StopCharacterMontage` _character _ch_shoot_standing))
            (`self.UpdateReticle` 0.5)
            (set `self.recoil pitch input` (`self.recoil pitch input_max`))
            (if (`self.firing`)
              (`KismetSystemLibrary.Delay` 1.0)
              (`GameplayStatics.PlaySoundAtLocation` "/Game/Audio/shell_falls.shell_falls" (+ (`self.K2_GetActorLocation`) (0.0 0.0 -80.0)) (struct) 1.0 1.0 0.0 null null null))))))))

(event `Emit Bullet`
  (`self.Emit Bullet M`
    (:`OutputPin`
      (`self.MakeNoise` 1.0 null (`self.K2_GetActorLocation`) (`self.Noise Range`) "1"))))

(event `self.Drop`
  (params (owner :type "Actor Object Reference"))
  (bind (_returnvalue_x _returnvalue_y _returnvalue_z) (`KismetMathLibrary.BreakVector` (`self.K2_GetActorLocation` owner)))
  (`self.K2_DetachFromActor` self "KeepWorld" "KeepWorld" "KeepWorld")
  (`self.K2_SetActorTransform` (`KismetMathLibrary.MakeTransform` (`KismetMathLibrary.MakeVector` _returnvalue_x _returnvalue_y (- _returnvalue_z 88.0))))
  (`self.Fire` false)
  (`self.SetInteractable` true))

(event `self.ToggleGun`
  (params (`equip/unequip` :type Boolean) (character :type "Actor Object Reference"))
  (bind _gun_widget (`self.gun widget`))
  (bind _gun_widget_2 (`self.gun widget`))
  (bind (_equipped_transform_location _equipped_transform_rotation) (`KismetMathLibrary.BreakTransform` (`self.equipped transform`)))
  (bind (_unequipped_transform_location _unequipped_transform_rotation) (`KismetMathLibrary.BreakTransform` (`self.unequipped transform`)))
  (bind _output_get (set `self.character` character))
  (bind _aimdeviationmultiplier (message `/Game/BP/CLM_BPI_Character.GetAimDeviationMultiplier` _output_get))
  (set `self.CharacterAimDeviationMultiplier` _aimdeviationmultiplier)
  (bind _output_get_2 (set `self.equipped` `equip/unequip`))
  (if `equip/unequip`
    (`KismetSystemLibrary.MoveComponentTo` (`self.gun mesh`) _equipped_transform_location _equipped_transform_rotation)
    (bind _yes_no (message `/Game/BP/CLM_BPI_Character.IsPlayer?` (`self.character`)))
    (if _yes_no
      (`/Engine/EditorBlueprintResources/StandardMacros.IsValid` (`self.gun widget`)
        (:`Is Valid`
          _)
        (:`Is Not Valid`
          (bind _returnvalue (`|CreateWidget` (`self.gun widget class`)))
          (set `self.gun widget` _returnvalue)))
      (`/Game/BP/UI/wdg_weapon.Init Weapon` _gun_widget (`self.weapon icon`))
      (`UserWidget.AddToViewport` _gun_widget 0))
    (bind _yes_no_2 (message `/Game/BP/CLM_BPI_Character.IsPlayer?` (`self.character`)))
    (if _yes_no_2
      (`/Engine/EditorBlueprintResources/StandardMacros.DoOnce` false
        (:`Completed`
          (`self.ReloadGun`)))
      (else
        (`/Engine/EditorBlueprintResources/StandardMacros.DoOnce` false
          (:`Completed`
            (`self.ReloadGun`)))))
    (else
      (`/Engine/EditorBlueprintResources/StandardMacros.IsValid` _gun_widget_2
        (:`Is Valid`
          (`Widget.RemoveFromParent` _gun_widget_2))
        (:`Is Not Valid`
          _))
      (`KismetSystemLibrary.MoveComponentTo` (`self.gun mesh`) _unequipped_transform_location _unequipped_transform_rotation))))

(event `self.ReloadGun`
  (bind _total_ammo_count (`self.total ammo count`))
  (bind _loaded_ammo_count (`self.loaded ammo count`))
  (bind _returnvalue (- _total_ammo_count (`self.magazin capacity`)))
  (set `self.total ammo count` (+ _total_ammo_count _loaded_ammo_count))
  (set `self.loaded ammo count` 0)
  (set `self.loaded ammo count` (`KismetMathLibrary.SelectInt` (`self.magazin capacity`) (+ _total_ammo_count _loaded_ammo_count) (> _returnvalue 0)))
  (set `self.total ammo count` (`KismetMathLibrary.Clamp` _returnvalue 0 (`self.max ammo count`)))
  (`self.UpdateAmmoCount`))

(event `self.player detector.OnComponentBeginOverlap`
  (params (OverlappedComponent :type "PrimitiveComponent Object Reference") (OtherActor :type "Actor Object Reference") (OtherComp :type "PrimitiveComponent Object Reference") (OtherBodyIndex :type Integer) (bFromSweep :type Boolean) (SweepResult :type "HitResult Structure (by ref)"))
  (bind _gun_mesh (`self.gun mesh`))
  (bind _returnvalue (`WidgetComponent.GetUserWidgetObject` (`self.PickupInfo`)))
  (bind _yes_no (message `/Game/BP/CLM_BPI_Character.IsPlayer?` OtherActor))
  (if _yes_no
    (`PrimitiveComponent.SetSimulatePhysics` _gun_mesh false)
    (`PrimitiveComponent.SetCollisionEnabled` _gun_mesh "NoCollision")
    (set `self.target character` OtherActor)
    (`self.EnableInput` (`GameplayStatics.GetPlayerController` 0))
    (bind (_gun_type _has_weapon_from_category) (message `/Game/BP/CLM_BPI_Character.GetWeaponFromCategory` OtherActor (`self.GunCategory`)))
    (message `/Game/BP/BPI_UI.PickupNew` _returnvalue _has_weapon_from_category)
    (bind _output_get (set `self.Display` true))
    (message `/Game/BP/BPI_UI.ShowTip` _returnvalue (select `/Game/BP/Guns/GunType` _gun_type :`NewEnumerator0` "/Game/BP/UI/UI_Assets/AK.AK" :`NewEnumerator1` "/Game/BP/UI/UI_Assets/revolver.revolver" :`NewEnumerator2` "/Game/BP/UI/UI_Assets/m16.m16" :`NewEnumerator3` "/Game/BP/UI/UI_Assets/pistol.pistol" :`NewEnumerator4` "/Game/BP/UI/UI_Assets/mp5.mp5" :`NewEnumerator5` "/Game/BP/UI/UI_Assets/rpg.rpg" :`NewEnumerator6` "/Game/BP/UI/UI_Assets/LMG.LMG" :`NewEnumerator7` "/Game/BP/UI/UI_Assets/m1870.m1870" :`NewEnumerator8` "/Game/AmplifyAnimationPack/Weapon/BP/UI/UI_Assets/shotgun.shotgun" :`NewEnumerator9` "/Game/AmplifyAnimationPack/Weapon/BP/UI/UI_Assets/uzi.uzi" :`NewEnumerator10` "/Game/BP/UI/UI_Assets/crossbow.crossbow" :`NewEnumerator11` "/Game/AmplifyAnimationPack/Weapon/BP/UI/UI_Assets/flamethrower.flamethrower" :`NewEnumerator12` "/Game/AmplifyAnimationPack/Weapon/BP/UI/UI_Assets/sniper.sniper" :!type "Texture2D Object Reference") (`self.weapon icon`) 5.0 _output_get)))

(event `self.player detector.OnComponentEndOverlap`
  (params (OverlappedComponent :type "PrimitiveComponent Object Reference") (OtherActor :type "Actor Object Reference") (OtherComp :type "PrimitiveComponent Object Reference") (OtherBodyIndex :type Integer))
  (bind _returnvalue (`WidgetComponent.GetUserWidgetObject` (`self.PickupInfo`)))
  (bind _yes_no (message `/Game/BP/CLM_BPI_Character.IsPlayer?` OtherActor))
  (if _yes_no
    (`self.DisableInput` null)
    (bind (_gun_type _has_weapon_from_category) (message `/Game/BP/CLM_BPI_Character.GetWeaponFromCategory` OtherActor (`self.GunCategory`)))
    (message `/Game/BP/BPI_UI.PickupNew` _returnvalue _has_weapon_from_category)
    (bind _output_get (set `self.Display` false))
    (message `/Game/BP/BPI_UI.ShowTip` _returnvalue (select `/Game/BP/Guns/GunType` _gun_type :`NewEnumerator0` "/Game/BP/UI/UI_Assets/AK.AK" :`NewEnumerator1` "/Game/BP/UI/UI_Assets/revolver.revolver" :`NewEnumerator2` "/Game/BP/UI/UI_Assets/m16.m16" :`NewEnumerator3` "/Game/BP/UI/UI_Assets/pistol.pistol" :`NewEnumerator4` "/Game/BP/UI/UI_Assets/mp5.mp5" :`NewEnumerator5` "/Game/BP/UI/UI_Assets/rpg.rpg" :`NewEnumerator6` "/Game/BP/UI/UI_Assets/LMG.LMG" :`NewEnumerator7` "/Game/BP/UI/UI_Assets/m1870.m1870" :`NewEnumerator8` "/Game/AmplifyAnimationPack/Weapon/BP/UI/UI_Assets/shotgun.shotgun" :`NewEnumerator9` "/Game/AmplifyAnimationPack/Weapon/BP/UI/UI_Assets/uzi.uzi" :`NewEnumerator10` "/Game/BP/UI/UI_Assets/crossbow.crossbow" :`NewEnumerator11` "/Game/AmplifyAnimationPack/Weapon/BP/UI/UI_Assets/flamethrower.flamethrower" :`NewEnumerator12` "/Game/AmplifyAnimationPack/Weapon/BP/UI/UI_Assets/sniper.sniper" :!type "Texture2D Object Reference") (`self.weapon icon`) 5.0 _output_get)))

(event `InputAction|interact`
  (params (Key :type "Key Structure"))
  (:`Pressed`
    (`self.SetInteractable` false)
    (`self.DisableInput` (`GameplayStatics.GetPlayerController` 0))
    (message `/Game/BP/CLM_BPI_Character.SwapGun` (`self.target character`) self)))

(event `self.SetInteractable`
  (params (enable :type Boolean))
  (bind _player_detector (`self.player detector`))
  (`/Engine/EditorBlueprintResources/StandardMacros.IsValid` _player_detector
    (:`Is Valid`
      (bind _output_get (set `PrimitiveComponent.bGenerateOverlapEvents` enable _player_detector))
      (`SceneComponent.SetVisibility` (`self.PickupInfo`) _output_get false))))

(event `DemoShoot`
  (bind _ns_flash (`self.NS_flash`))
  (`ActorComponent.Activate` _ns_flash true)
  (`KismetSystemLibrary.Delay` 1.0)
  (`ActorComponent.Deactivate` _ns_flash)
  (`self.DemoShoot`))

(event `self.SetReticleAccuracy`
  (params (`accuracy ` :type "Float (single-precision)"))
  (bind _reticle (`self.reticle`))
  (`/Engine/EditorBlueprintResources/StandardMacros.IsValid` _reticle
    (:`Is Valid`
      (`/Game/BP/UI/Reticle/Wdg_Reticle.SetAccuracy` _reticle `accuracy `))))

(event `self.ActiveReload`
  (bind _gun_mesh (`self.gun mesh`))
  (bind _gun_reload_standing (`self.gun_reload_standing`))
  (bind _character (`self.character`))
  (if (not (== (`self.loaded ammo count`) (`self.magazin capacity`)))
    (bind _reload_delay (message `/Game/BP/CLM_BPI_Character.Reload` _character))
    (bind _newparam (message `/Game/BP/CLM_BPI_Character.GetMovementMode` _character))
    (`MeshComponent.SetScalarParameterValueOnMaterials` _gun_mesh "mask" 1.0)
    (bind _returnvalue (select `/Game/BP/SoldierMovementMode` _newparam :`NewEnumerator0` _gun_reload_standing :`NewEnumerator1` _gun_reload_standing :`NewEnumerator2` _gun_reload_standing :`NewEnumerator3` (`self.gun_reload_crouching`) :`NewEnumerator4` (`self.gun_reload_prone`)))
    (`|PlayMontage` _gun_mesh _returnvalue
      (:`then`
        (set `self.reloading` true)
        (`KismetSystemLibrary.PrintString` (`KismetSystemLibrary.GetDisplayName` _returnvalue))
        (`KismetSystemLibrary.Delay` _reload_delay)
        (set `self.reloading` false)
        (`self.ReloadGun`)))))

(fn `GetBulletTarget`
  (returns (target :type "Vector Structure"))
  (bind _target_point (`self.target point`))
  (bind _target (message `/Game/BP/CLM_BPI_Character.GetTargetLocation` (`self.character`)))
  (bind (_outhit _returnvalue) (`KismetSystemLibrary.LineTraceSingle` (`SceneComponent.GetSocketLocation` (`self.gun mesh`) "nozzle") _target "TraceTypeQuery1"))
  (if _returnvalue
    (`SceneComponent.K2_SetRelativeLocation` _target_point (`KismetMathLibrary.MakeVector` (`.Distance` (`GameplayStatics.BreakHitResult` _outhit))) false false)
    (else
      (`SceneComponent.K2_SetRelativeLocation` _target_point (2000.0 0.0 0.0) false false)))
  (return (`SceneComponent.K2_GetComponentLocation` (`self.target point`))))

(fn `GetCategory`
  (returns (`gun category` :type "/Game/BP/Guns/GunCategory Enum"))
  (return (`self.GunCategory`)))

(fn `GetGunType`
  (returns (`gun type` :type "/Game/BP/Guns/GunType Enum"))
  (return (`self.GunType`)))

(fn `GetReloadAnimations`
  (returns (standing :type "AnimMontage Object Reference") (crouching :type "AnimMontage Object Reference") (proning :type "AnimMontage Object Reference"))
  (return (`self.ch_reload_standing`) (`self.ch_reload_crouching`) (`self.ch_reload_proning`)))

(fn `GetShootAnimation`
  (returns (`shoot animation` :type "AnimMontage Object Reference"))
  (return (`self.ch_shoot_standing`)))

(fn `GetWeaponSocket`
  (params (`socket name` :type Name))
  (returns (`socket transform` :type "Transform Structure"))
  (return (`SceneComponent.GetSocketTransform` (`self.gun mesh`) `socket name` "RTS_World")))

(fn `IsEquipped`
  (returns (`yes/no` :type Boolean))
  (return (`self.equipped`)))

(fn `UpdateAmmoCount`
  (bind _gun_widget (`self.gun widget`))
  (`/Engine/EditorBlueprintResources/StandardMacros.IsValid` _gun_widget
    (:`Is Valid`
      (`/Game/BP/UI/wdg_weapon.Update Ammo Count` _gun_widget (`self.total ammo count`) (`self.loaded ammo count`)))))

(fn `UpdateReticle`
  (params (accuracy :type "Float (double-precision)"))
  (`self.SetReticleAccuracy` accuracy))

(fn `UserConstructionScript`)