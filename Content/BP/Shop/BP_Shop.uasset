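; BP_Shop is a shop actor that lets the player open a shop menu while standing inside its box trigger.
; On overlap it shows an interact key tip on the HUD and enables input, which it disables when the player leaves.
; Interact lazily creates and reuses WDG_Shop, hands it a self reference and switches to UI-only input with a cursor.
; A SpawnActor event spawns a given class at a given transform, adjusting for collisions.
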(event `self.Box.OnComponentBeginOverlap`
  (params (OverlappedComponent :type "PrimitiveComponent Object Reference") (OtherActor :type "Actor Object Reference") (OtherComp :type "PrimitiveComponent Object Reference") (OtherBodyIndex :type Integer) (bFromSweep :type Boolean) (SweepResult :type "HitResult Structure (by ref)"))
  (bind _returnvalue (`GameplayStatics.GetPlayerController` 0))
  (bind _yes_no (message `/Game/BP/CLM_BPI_Character.IsPlayer?` OtherActor))
  (if _yes_no
    (bind _keys (message `/Game/BP/CLM_BPI_PlayerController.GetInput` _returnvalue "interact"))
    (message `/Game/BP/BPI_UI.ShowTip` (`PlayerController.GetHUD` _returnvalue) (`KismetStringLibrary.Concat_StrStr` "Press <input>" _keys "</> to Shop") 5.0)
    (`self.EnableInput` (`GameplayStatics.GetPlayerController` 0))))

(event `self.Box.OnComponentEndOverlap`
  (params (OverlappedComponent :type "PrimitiveComponent Object Reference") (OtherActor :type "Actor Object Reference") (OtherComp :type "PrimitiveComponent Object Reference") (OtherBodyIndex :type Integer))
  (bind _yes_no (message `/Game/BP/CLM_BPI_Character.IsPlayer?` OtherActor))
  (if _yes_no
    (`self.DisableInput` (`GameplayStatics.GetPlayerController` 0))))

(event `InputAction|interact`
  (params (Key :type "Key Structure"))
  (bind _returnvalue (`GameplayStatics.GetPlayerController` 0))
  (bind _wdg_shop (`self.WDG_Shop`))
  (:`Pressed`
    (`/Engine/EditorBlueprintResources/StandardMacros.IsValid` (`self.WDG_Shop`)
      (:`Is Valid`
        _)
      (:`Is Not Valid`
        (bind _returnvalue_2 (`|CreateWidget` "/Game/BP/Shop/WDG_Shop.WDG_Shop_C"))
        (bind _output_get (set `self.WDG_Shop` _returnvalue_2))
        (set `/Game/BP/Shop/WDG_Shop.BP_Shop` self _output_get)))
    (if (not (`Widget.IsInViewport` _wdg_shop))
      (`UserWidget.AddToViewport` _wdg_shop 0)
      (`WidgetBlueprintLibrary.SetInputMode_UIOnlyEx` _returnvalue null)
      (set `PlayerController.bShowMouseCursor` true _returnvalue))))

(event `Spawn Actor`
  (params (Class :type "Actor Class Reference") (SpawnTransform :type "Transform Structure"))
  (`|SpawnActorFromClass` Class SpawnTransform "AdjustIfPossibleButAlwaysSpawn" "OverrideRootScale" null null))

(fn `UserConstructionScript`)