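; Shooting target that flips between upright and cover poses, optionally hiding on a timer or sliding side to side.
; BeginPlay starts the enabled loops: HideLoop alternates poses, while MoveLoop raises the target, slides it to alternating ±MoveRange, then takes cover.
; Two Move target macro instances drive the slide, with duration scaled by range.
; The first damaging OnBulletHit sets Destroyed to end the loops, stops movement and rotates the target down.
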(event `self.ReceiveBeginPlay`
  (if (`self.hide loop enabled`)
    (`self.HideLoop`))
  (if (`self.move loop enabled`)
    (`self.MoveLoop`)))

(event `OnBulletHit_E`
  (params (damage :type "Float (double-precision)") (hitLocation :type "Vector Structure"))
  (if (> damage 0.0)
    (`/Engine/EditorBlueprintResources/StandardMacros.DoOnce` false
      (:`Completed`
        (set `self.destroyed` true)
        (`self.interrupt`)
        (`KismetSystemLibrary.MoveComponentTo` (`self.shootTarget`) (0.0 0.0 0.0) (struct :`Yaw` 90.0 :`Roll` 90.0) true false 0.2 true)))))

(event `ToggleCover`
  (params (`take cover` :type Boolean))
  (bind _shoottarget (`self.shootTarget`))
  (`KismetSystemLibrary.MoveComponentTo` _shoottarget (`SceneComponent.RelativeLocation` _shoottarget) (`KismetMathLibrary.MakeRotator` (`KismetMathLibrary.SelectFloat` 90.0 0.0 `take cover`) 0.0 90.0) true false 0.2 true))

(event `HideLoop`
  (`KismetSystemLibrary.Delay` (`self.hide start delay`))
  (if (not (`self.destroyed`)) :!label _label
    (`/Engine/EditorBlueprintResources/StandardMacros.FlipFlop`
      (:`A`
        (`self.ToggleCover` true))
      (:`B`
        (`self.ToggleCover` false)))
    (`KismetSystemLibrary.Delay` (`self.cover delay`))
    (goto _label)))

(event `MoveLoop`
  (if (not (`self.destroyed`)) :!label _label_2
    (`self.ToggleCover` false)
    (`KismetSystemLibrary.Delay` 0.4)
    (`/Engine/EditorBlueprintResources/StandardMacros.FlipFlop`
      (:`A`
        (`self.Move target` (`self.move range`) :!label _label_3))
      (:`B`
        (`self.Move target` (* (`self.move range`) -1.0) :!label _label_4)))
    (`self.ToggleCover` true)
    (`KismetSystemLibrary.Delay` (`self.cover delay`))
    (goto _label_2)))

(event `interrupt`
  (`|ExecutionSequence`
    (:`then_0`
      (goto _label_3 :!via `Stop`))
    (:`then_1`
      (goto _label_4 :!via `Stop`))))

(fn `OnBulletHit`
  (params (damage :type "Float (double-precision)") (hitLocation :type "Vector Structure") (`shooter location` :type "Vector Structure"))
  (returns (headshot :type Boolean))
  (`self.OnBulletHit_E` damage hitLocation)
  (return false))

(fn `UserConstructionScript`)