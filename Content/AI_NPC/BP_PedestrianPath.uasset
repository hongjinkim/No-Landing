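; BP_PedestrianPath is a pedestrian path actor that spawns NPC_Point actors along its Path spline on BeginPlay.
; PlaceNPCPoints loops by distance at a fixed interval until the spline length is reached, storing each point in NpcPoint and printing the running distance.
; Before spawning, it calls SetLifeSpan with zero on stored points, which clears their lifespan rather than destroying them, then empties the array.
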(event `self.ReceiveBeginPlay`
  (`self.Place NPC Points`))

(event `Place NPC Points`
  (set `self.Distance` 0.0)
  (for _array_element (`self.npc_point`)
    (`self.SetLifeSpan` _array_element 0.0))
  (`KismetArrayLibrary.Array_Clear` (`self.npc_point`))
  (bind _returnvalue (`|SpawnActorFromClass` "/Game/AI_NPC/NPC_Point.NPC_Point_C" (`KismetMathLibrary.MakeTransform` (`SplineComponent.GetLocationAtDistanceAlongSpline` (`self.path`) (`self.Distance`) "World")) "Undefined" "OverrideRootScale" null null :!label _label))
  (`KismetArrayLibrary.Array_Add` (`self.npc_point`) _returnvalue)
  (bind _output_get (set `self.Distance` (+ (`self.Distance`) 400.0)))
  (`KismetSystemLibrary.PrintString` (`KismetStringLibrary.Conv_DoubleToString` _output_get))
  (if (< _output_get (`SplineComponent.GetSplineLength` (`self.path`)))
    (goto _label)))

(fn `UserConstructionScript`)