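; Behavior tree task that sends the AI pawn to a random reachable point near the player character.
; It starts an AI MoveTo and finishes successfully after a fixed delay from the move request, without waiting for arrival.
; The debug print re-evaluates the random point, so it can differ from the actual destination.
; Elapsed time and run count are tracked but never affect the result.
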(event `self.ReceiveTickAI`
  (params (OwnerController :type "AIController Object Reference") (ControlledPawn :type "Pawn Object Reference") (DeltaSeconds :type "Float (single-precision)"))
  (set `self.MovingTime` (+ (`self.MovingTime`) DeltaSeconds)))

(event `self.ReceiveExecuteAI`
  (params (OwnerController :type "AIController Object Reference") (ControlledPawn :type "Pawn Object Reference"))
  (bind _randomlocation (`NavigationSystemV1.K2_GetRandomReachablePointInRadius` (`Actor.K2_GetActorLocation` (`GameplayStatics.GetPlayerCharacter` 0)) 500.0 null null))
  (`KismetSystemLibrary.PrintString` (`KismetStringLibrary.Conv_VectorToString` _randomlocation))
  (`|AIMoveTo` ControlledPawn _randomlocation null 100.0 true
    (:`then`
      (`KismetSystemLibrary.Delay` 2.0)
      (set `self.count` (+ (`self.count`) 1))
      (set `self.MovingTime` 0.0)
      (`self.FinishExecute` true))))