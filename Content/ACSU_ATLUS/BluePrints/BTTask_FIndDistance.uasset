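; Behavior Tree task that measures the distance from the AI-controlled pawn to player character 0.
; On execute it takes the length of the vector between the two actor locations and writes it as a float to the blackboard key named Distasnce.
; It then prints a Korean debug message saying the value was saved and immediately finishes as successful.
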(event `self.ReceiveExecuteAI`
  (params (OwnerController :type "AIController Object Reference") (ControlledPawn :type "Pawn Object Reference"))
  (bind _output_get (set `self.Distance` (`KismetMathLibrary.VSize` (- (`Actor.K2_GetActorLocation` (`GameplayStatics.GetPlayerCharacter` 0)) (`Actor.K2_GetActorLocation` ControlledPawn)))))
  (`BTFunctionLibrary.SetBlackboardValueAsFloat` (`self.Distasnce`) _output_get)
  (`KismetSystemLibrary.PrintString` "값 저장됨")
  (`self.FinishExecute` true))