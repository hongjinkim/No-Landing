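; BP_Boss is the ACSU Atlus boss character, which plays an activation montage on spawn and tracks HP.
; Damage lowers HP and, at zero, plays the death montage and flags it dead.
; FireRocket spawns a BP_Rocket at the capsule's Muzzle socket and sends it a launch message.
; The construction script slaves the gun, handspad and mine meshes to the body's pose; box overlaps only print debug text.
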(event `self.ReceiveBeginPlay`
  (bind _returnvalue (`self.PlayAnimMontage` "/Game/ACSU_ATLUS/Animations/A_ACSU_Atlus_Activation_Montage.A_ACSU_Atlus_Activation_Montage"))
  (`KismetSystemLibrary.Delay` _returnvalue))

(event `self.ReceiveAnyDamage`
  (params (Damage :type "Float (single-precision)") (DamageType :type "DamageType Object Reference") (InstigatedBy :type "Controller Object Reference") (DamageCauser :type "Actor Object Reference"))
  (bind _hp (`self.HP`))
  (if (not (`self.IsDead`))
    (bind _output_get (set `self.HP` (- _hp Damage)))
    (`KismetSystemLibrary.PrintString` (`KismetStringLibrary.Conv_DoubleToString` _output_get))
    (if (<= _hp 0.0)
      (`self.PlayAnimMontage` "/Game/ACSU_ATLUS/Animations/A_ACSU_Atlus_Dead_Montage.A_ACSU_Atlus_Dead_Montage")
      (set `self.IsDead` true))))

(event `self.Box.OnComponentBeginOverlap`
  (params (OverlappedComponent :type "PrimitiveComponent Object Reference") (OtherActor :type "Actor Object Reference") (OtherComp :type "PrimitiveComponent Object Reference") (OtherBodyIndex :type Integer) (bFromSweep :type Boolean) (SweepResult :type "HitResult Structure (by ref)"))
  (`KismetSystemLibrary.PrintString` (`KismetSystemLibrary.GetDisplayName` OverlappedComponent)))

(event `FireRocket`
  (bind _returnvalue (`|SpawnActorFromClass` "/Game/ACSU_ATLUS/BluePrints/BP_Rocket.BP_Rocket_C" (`KismetMathLibrary.Conv_VectorToTransform` (`SceneComponent.GetSocketLocation` (`self.CapsuleComponent`) "Muzzle")) "Undefined" "OverrideRootScale" null null))
  (message `/Game/ACSU_ATLUS/BluePrints/BPi_Boss.LaunchMissile` _returnvalue))

(fn `UserConstructionScript`
  (`SkinnedMeshComponent.SetLeaderPoseComponent` (`self.Gun1_R`) (`self.Mesh`) false)
  (`SkinnedMeshComponent.SetLeaderPoseComponent` (`self.Gun1_L`) (`self.Mesh`) false)
  (`SkinnedMeshComponent.SetLeaderPoseComponent` (`self.Gun2_R`) (`self.Mesh`) false)
  (`SkinnedMeshComponent.SetLeaderPoseComponent` (`self.Gun2_L`) (`self.Mesh`) false)
  (`SkinnedMeshComponent.SetLeaderPoseComponent` (`self.Handspad_R`) (`self.Mesh`) false)
  (`SkinnedMeshComponent.SetLeaderPoseComponent` (`self.Handspad_L`) (`self.Mesh`) false)
  (`SkinnedMeshComponent.SetLeaderPoseComponent` (`self.Mines_R`) (`self.Mesh`) false)
  (`SkinnedMeshComponent.SetLeaderPoseComponent` (`self.Mines_L`) (`self.Mesh`) false))